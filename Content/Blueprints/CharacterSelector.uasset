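; CharacterSelector is an actor for character skin selection that swaps between the Joyce and JoycePink components.
; Each selection event sets the skin index and toggles both components' visibility inversely from its Selected flag.
; Both then pass the skin index and BlueOrRed value to the game instance through a save message.
; Code that creates the selection widget and links it back to this actor is present but disconnected.
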(event Custom|Udate%20Character%20Data
  (Class|InstanceInterface|SaveCharacterData(Message) (Game|GetGameInstance) (Variables|Default|GetBlue%20Or%20Red) (Variables|Default|GetSelected%20Skin)))

(event Custom|Selected%20Pink
  (params (Selected :type Boolean))
  (Variables|Default|SetSelected%20Skin 1)
  (Rendering|SetVisibility (Variables|Default|GetJoyce) Selected false)
  (Rendering|SetVisibility (Variables|Default|GetJoyce_Pink) (not Selected) false)
  (CallFunction|UdateCharacterData))

(event Custom|joyce%20selected
  (params (selected :type Boolean))
  (Variables|Default|SetSelected%20Skin 0)
  (Rendering|SetVisibility (Variables|Default|GetJoyce) (not selected) false)
  (Rendering|SetVisibility (Variables|Default|GetJoyce_Pink) selected false)
  (CallFunction|UdateCharacterData))

(event EventBeginPlay)

(event Collision|EventActorBeginOverlap
  (params (OtherActor :type Actor%20Object%20Reference)))

(event EventTick
  (params (DeltaSeconds :type Float%20%28single-precision%29)))

(fn ConstructionScript)