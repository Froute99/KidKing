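; Player controller for the KidKing game that handles character selection, spawning and a debug scoreboard.
; After login it adds a character selection widget to the player's screen.
; RPC_SpawnPlayer passes the chosen character index and team index to BP_KidKingGameMode, then possesses the returned pawn.
; Pressing Tab prints the ID and score from the player state of each controller in the game mode's list.
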(event Custom|RPC_SpawnPlayer
  (params (Character%20Index :type Integer))
  ;[0 0 0] Spawn Player
  (Variables|Default|SetCharacter%20Index Character%20Index)
  (if (Pawn|IsLocalPlayerController)
    _
    (else
      _))
  (bind _asbp_kid_king_game_mode (Utilities|Casting|CastToBP_KidKingGameMode (Game|GetGameMode)))
  (bind _returnvalue (Default|SpawnPlayer _asbp_kid_king_game_mode self (Variables|Default|GetCharacter%20Index) (Variables|Default|GetTeamIndex)))
  (Pawn|Possess self _returnvalue))

(event Custom|OnPostLogin
  ;[0 0 0] Spawn Player
  (bind _returnvalue (UserInterface|CreateWidget "/Game/Blueprints/UI/BP_WDG_CharacterSelection.BP_WDG_CharacterSelection_C" self))
  (UserInterface|Viewport|AddtoPlayerScreen _returnvalue))

(event Custom|ScoreBoard
  (bind _asbp_kid_king_game_mode (Utilities|Casting|CastToBP_KidKingGameMode (Game|GetGameMode)))
  (Utilities|FlowControl|Sequence
    (:then_0
      (for _array_element (Variables|/Game/Blueprints/Core/BP_KidKingGameMode.BP_KidKingGameMode_C|GetPCs _asbp_kid_king_game_mode)
        (bind _asbp_kid_king_player_state (Utilities|Casting|CastToBP_KidKingPlayerState (Variables|/Script/Engine.Controller|GetPlayerState _array_element)))
        (Development|PrintString (Utilities|String|ToString(Text) (Utilities|Text|FormatText "ID: {id}    Score: {score}" (Variables|/Script/Engine.PlayerState|GetPlayerId _asbp_kid_king_player_state) (Variables|/Game/Blueprints/Character/BP_KidKingPlayerState.BP_KidKingPlayerState_C|GetPlayerScore _asbp_kid_king_player_state)))))
      ;[1 1 1] New Line
      (Development|PrintString ""))))

(event EventBeginPlay
  ;[0 0 0] Spawn Player
)

(event Input|KeyboardEvents|Tab
  (params (Key :type Key%20Structure))
  (:Pressed
    (CallFunction|ScoreBoard)))

(fn ConstructionScript)