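; BP_Thrust is the hit-detection actor for Joyce's thrust ability, using the Gameplay Ability System.
; Each tick it snaps to its owner's location and rotation.
; The first capsule overlap with another actor's valid ability system applies GE_Thrust from the owner and sends that actor a Character.Damaged event.
; A DoOnce with no reset limits each instance to one hit, and the cached Joyce reference is unused.
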(event OnComponentBeginOverlap(Capsule)
  (params (OverlappedComponent :type Primitive%20Component%20Object%20Reference) (OtherActor :type Actor%20Object%20Reference) (OtherComp :type Primitive%20Component%20Object%20Reference) (OtherBodyIndex :type Integer) (bFromSweep :type Boolean) (SweepResult :type Hit%20Result%20Structure%20%28by%20ref%29))
  (bind _returnvalue (Ability|GetAbilitySystemComponent OtherActor))
  (if (!= (Ability|GetAbilitySystemComponent (Components|GetOwner)) (Ability|GetAbilitySystemComponent OtherActor))
    (Utilities|IsValid _returnvalue
      (:Is%20Valid
        (Utilities|FlowControl|DoOnce false
          (:Completed
            (GameplayEffects|ApplyGameplayEffectToTarget :self (Ability|GetAbilitySystemComponent (Components|GetOwner)) :GameplayEffectClass "/Game/Blueprints/Character/Joyce/Ability/Effects/GE_Thrust.GE_Thrust_C" :Target _returnvalue)
            (Ability|SendGameplayEventtoActor OtherActor "(TagName=\"Character.Damaged\")" (Utilities|Struct|MakeGameplayEventData "(TagName=\"\")" self OtherActor 0 0 "()" "(GameplayTags=)" "(GameplayTags=)" 0.0 (Ability|TargetData|AbilityTargetDatafromActor OtherActor)))))))))

(event EventBeginPlay
  (bind _outactors (Actor|GetAllActorsOfClass "/Game/Blueprints/Character/Joyce/BP_Joyce.BP_Joyce_C"))
  (Variables|Default|SetCharacter_REF (Utilities|Array|Get(acopy) _outactors)))

(event Collision|EventActorBeginOverlap
  (params (OtherActor :type Actor%20Object%20Reference)))

(event EventTick
  (params (DeltaSeconds :type Float%20%28single-precision%29))
  (bind _returnvalue (Components|GetOwner))
  (bind _returnvalue_2 (Transformation|GetActorLocation _returnvalue))
  (Transformation|SetActorLocation (Math|Vector|MakeVector (.x _returnvalue_2) (.y _returnvalue_2) (.z _returnvalue_2)) false false)
  (Transformation|SetActorRotation (Transformation|GetActorRotation _returnvalue)))

(fn ConstructionScript)