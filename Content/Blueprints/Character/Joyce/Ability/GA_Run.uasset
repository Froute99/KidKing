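; GA_Run is a Gameplay Ability for the Joyce character that makes the avatar run by raising its maximum walk speed.
; On activation it commits, then casts the actor info's movement component to CharacterMovementComponent and sets a fixed MaxWalkSpeed.
; It prints the new speed and ends immediately without restoring the old one, as OnEndAbility is empty.
; A failed cast only prints a debug string and leaves the ability active.
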(event Custom|OnCommitAbility
  (bind _ascharacter_movement_component (Utilities|Casting|CastToCharacterMovementComponent (.MovementComponent (Utilities|Struct|BreakGameplayAbilityActorInfo (Ability|GetActorInfo))))
    (:then
      (bind _output_get (Variables|/Script/Engine.CharacterMovementComponent|SetMaxWalkSpeed _ascharacter_movement_component 1.2e+03))
      (Development|PrintString (Utilities|String|ToString(Float) _output_get))
      (Ability|EndAbility))
    (:CastFailed
      (Development|PrintString "Hello"))))

(event Ability|EventActivateAbility
  (Ability|CommitAbility)
  (CallFunction|OnCommitAbility))

(event Ability|EventOnEndAbility
  (params (bWasCancelled :type Boolean)))