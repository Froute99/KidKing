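; Joyce, a playable sword character with combo attacks, dodge, guard, Thrust and Slash skills, power-up buff and death handling.
; Input activates Gameplay Ability System abilities by tag or applies effects, while events play montages, drive lunge velocity through timelines and spawn skill actors.
; A looping-timer socket line trace damages one target per swing, and gameplay events trigger hit reactions and buffs.
; Death spawns score balls and UI; debug keys are included.
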(event Custom|RPC_AnyDamage
  ;[1 1 1] Damaged
  (if (> (Class|BaseCharacter|GetHealth) 0.0)
    (Animation|PlayAnimMontage "/Game/Blueprints/Character/Joyce/Animation/Montage/AM_Joyce_Hit.AM_Joyce_Hit" 1.0 "None")))

(event Custom|CamShake
  ;[1 1 1] CamShake
)

(event Custom|Btn%20Attack
  (bind _mesh (Variables|Character|GetMesh))
  ;[1 1 1] Default Attack
  ;;[0 0 0] Combo
  (if (Variables|Default|GetIsBtnAttack)
    (Variables|Default|SetIsBtnAttack false)
    (if (>= (Class|BaseCharacter|GetStamina) 4.0)
      (GameplayEffects|ApplyGameplayEffectToSelf :self (Variables|Default|GetAbilitySystemComponent) :GameplayEffectClass "/Game/Blueprints/Character/Joyce/Ability/Effects/GE_AttackCost.GE_AttackCost_C")
      (switch int (Variables|Default|GetComboIndex)
        (:0
          (Variables|Default|SetComboIndex 1)
          (Variables|Default|SetComboMoveDistance 1.5e+02)
          (Animation|Montage|PlayMontage _mesh "/Game/Blueprints/Character/Joyce/Animation/Montage/AM_Combo1.AM_Combo1"
            (:then
              (Timeline|Timeline PlayFromStart
                (:Update
                  (Variables|/Script/Engine.MovementComponent|SetVelocity (Variables|Character|GetCharacterMovement) (Math|Vector|MakeVector (.x (* (Transformation|GetActorForwardVector) (Variables|Default|GetComboMoveDistance))) (.y (* (Transformation|GetActorForwardVector) (Variables|Default|GetComboMoveDistance))) (.z (Variables|/Script/Engine.MovementComponent|GetVelocity (Variables|Character|GetCharacterMovement))))))))
            (:OnInterrupted
              (Utilities|FlowControl|RetriggerableDelay 0.8 :!label _label)
              (CallFunction|UpdateNotify))))
        (:1
          (Variables|Default|SetComboIndex 2)
          (Variables|Default|SetComboMoveDistance 1e+03)
          (Animation|Montage|PlayMontage _mesh "/Game/Blueprints/Character/Joyce/Animation/Montage/AM_Combo2.AM_Combo2"
            (:then
              (Timeline|Timeline PlayFromStart))
            (:OnInterrupted
              (goto _label))))
        (:2
          (Variables|Default|SetComboIndex 3)
          (Variables|Default|SetComboMoveDistance 0.0)
          (Animation|Montage|PlayMontage _mesh "/Game/Blueprints/Character/Joyce/Animation/Montage/AM_Combo3.AM_Combo3"
            (:then
              (Timeline|Timeline PlayFromStart))
            (:OnInterrupted
              (goto _label))))
        (:3
          (Variables|Default|SetComboIndex 0)
          (Variables|Default|SetComboMoveDistance 1e+03)
          (Animation|Montage|PlayMontage _mesh "/Game/Blueprints/Character/Joyce/Animation/Montage/AM_Combo4.AM_Combo4"
            (:then
              (Timeline|Timeline PlayFromStart))
            (:OnInterrupted
              (goto _label)))))
      (else
        (Variables|Default|SetIsAttackingCombo false)))))

(event Custom|OnGuardServer
  ;[1 1 1] Guard
  (CallFunction|OnGuard))

(event Custom|OffGuardSever
  ;[1 1 1] Guard
  (CallFunction|OffGuard))

(event Custom|ResetCombo
  ;[1 1 1] Default Attack
  ;;[0 0 0] Combo
  (Variables|Default|SetIsAttackingCombo false)
  (Variables|Default|SetIsBtnAttack false)
  (Variables|Default|SetComboIndex 0))

(event Custom|Client%20Death
  ;[1 1 1] Die
  (Variables|Default|SetIsDead true))

(event Custom|SwordLineTrace
  (bind _staticmesh (Variables|Default|GetStaticMesh))
  ;[1 1 1] Default Attack
  (bind _outhit (Collision|LineTraceByChannel (Transformation|GetSocketLocation _staticmesh "BottomSocket") (Transformation|GetSocketLocation _staticmesh "TopSocket") "TraceTypeQuery3" false 0 "ForDuration"))
  (Utilities|IsValid (Ability|GetAbilitySystemComponent (.HitActor (Collision|BreakHitResult _outhit)))
    (:Is%20Valid
      (Utilities|FlowControl|DoOnce false
        (:Completed
          (GameplayEffects|ApplyGameplayEffectToTarget :self (Ability|GetAbilitySystemComponent self) :GameplayEffectClass "/Game/Blueprints/Character/Joyce/Ability/Effects/GE_DamageSample.GE_DamageSample_C" :Target (Ability|GetAbilitySystemComponent (.HitActor (Collision|BreakHitResult _outhit))))
          (Ability|SendGameplayEventtoActor (.HitActor (Collision|BreakHitResult _outhit)) "(TagName=\"Character.Damaged\")" (Utilities|Struct|MakeGameplayEventData "(TagName=\"\")" self (.HitActor (Collision|BreakHitResult _outhit)) 0 0 "()" "(GameplayTags=)" "(GameplayTags=)" 0.0 (Ability|TargetData|AbilityTargetDatafromActor (.HitActor (Collision|BreakHitResult _outhit))))))))))

(event Custom|OnThrust
  (bind _returnvalue (Transformation|GetActorLocation))
  (bind _returnvalue_2 (Transformation|GetActorForwardVector))
  (bind _spiraldistance (Variables|Default|GetSpiralDistance))
  (bind _returnvalue_3 (* _returnvalue_2 _spiraldistance))
  ;[1 1 1] Debug Key
  ;;[0 0 0] Thrust
  (Animation|Montage|PlayMontage (Variables|Character|GetMesh) "/Game/Blueprints/Character/Joyce/Animation/Montage/AM_JoyceSpiralSkill.AM_JoyceSpiralSkill"
    (:then
      (Audio|PlaySoundatLocation "/Game/resource/Sound/Attack/Slash.Slash" "0, 0, 0" "0, 0, 0" 1.0 1.0 3.5 0 0 0 0)
      (Utilities|FlowControl|Delay 0.3)
      (bind _returnvalue_4 (Game|SpawnActorfromClass "/Game/Blueprints/Character/Joyce/Ability/BP_Thrust.BP_Thrust_C" (Math|Transform|MakeTransform (Math|Vector|MakeVector (.x _returnvalue) (.y _returnvalue) (.z _returnvalue)) (Transformation|GetActorRotation)) "Undefined" self 0))
      (Input|DisableInput 0)
      (Timeline|Timeline_0 PlayFromStart
        (:Update
          (Variables|/Script/Engine.MovementComponent|SetVelocity (Variables|Character|GetCharacterMovement) (Math|Vector|MakeVector (.x _returnvalue_3) (.y _returnvalue_3) (.z (Variables|/Script/Engine.MovementComponent|GetVelocity (Variables|Character|GetCharacterMovement)))))
          (Utilities|FlowControl|Delay 1.0)
          (Actor|DestroyActor _returnvalue_4)
          (Input|EnableInput 0))))))

(event Custom|UpdateNotify
  ;[1 1 1] Default Attack
  (CallFunction|StopTriggerSword)
  (Input|EnableInput 0)
  (CallFunction|ResetCombo))

(event Custom|Server%20Death
  ;[1 1 1] Die
  (Variables|Default|SetIsDead true))

(event Custom|Dodge
  ;[1 1 1] Dodge
  (CallFunction|DodgeRPC))

(event Custom|RPC_DebugHit
  ;[1 1 1] Debug Key
  ;;[0 0 0] Debug Hit
  (GameplayEffects|ApplyGameplayEffectToSelf :self (Variables|Default|GetAbilitySystemComponent) :GameplayEffectClass "/Game/Blueprints/Character/Joyce/Ability/Effects/GE_DamageSample.GE_DamageSample_C")
  (Ability|SendGameplayEventtoActor self "(TagName=\"Character.Damaged\")" (Utilities|Struct|MakeGameplayEventData "(TagName=\"Character.Damaged\")" self)))

(event Custom|PowerBuffRecv
  ;[1 1 1] Powerup Buff
  (CallFunction|PowerBuffRecvREP))

(event Custom|IncreaseTime
  (bind _asbp_game_state (Utilities|Casting|CastToBP_GameState (Game|GetGameState)))
  (Default|IncreaseTime _asbp_game_state))

(event Custom|PowerBuffRecv_REP
  ;[1 1 1] Powerup Buff
  (GameplayEffects|ApplyGameplayEffectToSelf :self (Variables|Default|GetAbilitySystemComponent) :GameplayEffectClass "/Game/Blueprints/Character/Joyce/Ability/Effects/GE_PowerUp.GE_PowerUp_C")
  (Utilities|FlowControl|DoOnce false :!label _label
    (:Completed
      (bind _returnvalue (Niagara|SpawnSystemAttached "/Game/resource/Buff_NS/STRBuff_NS.STRBuff_NS" (Variables|Character|GetMesh) "None" "0, 0, 0" "0, 0, 0" "KeepRelativeOffset" false))
      (Utilities|FlowControl|Delay (Variables|Default|GetBuffDuration))
      (GameplayEffects|RemoveActiveEffectswithTags (Variables|Default|GetAbilitySystemComponent) "(GameplayTags=((TagName=\"Test.Buff\")))")
      (Components|DestroyComponent _returnvalue)
      (goto _label Reset))))

(event Custom|ScoreBall
  ;[1 1 1] Score
  (if (not (== (Variables|Default|GetScoreIndex) 5)) :!label _label
    (Utilities|FlowControl|Delay 0.2)
    (Game|SpawnActorfromClass "/Game/Blueprints/Score/BP_ScoreBall.BP_ScoreBall_C" (Math|Transform|MakeTransform (.location (Transformation|GetWorldTransform (Variables|Default|GetScore))) (Math|Rotator|MakeRotator 0.0 0.0 (.yaw (Math|Random|RandomRotator false))) "1.000000,1.000000,1.000000") "Undefined" 0 3e+02 0.5 0)
    (Variables|Default|SetScoreIndex (+ (Variables|Default|GetScoreIndex) 1))
    (goto _label)))

(event Custom|Dodge_RPC
  (bind _returnvalue (Transformation|GetActorForwardVector))
  (bind _movedistance (Variables|Default|GetMoveDistance))
  (bind _returnvalue_2 (* _returnvalue _movedistance))
  ;[1 1 1] Dodge
  (Animation|Montage|PlayMontage (Variables|Character|GetMesh) "/Game/Blueprints/Character/Joyce/Animation/Montage/AM_Rolling.AM_Rolling"
    (:then
      ;;[1 1 1] Don't Used
      (Timeline|Movement PlayFromStart
        (:Update
          (Variables|/Script/Engine.MovementComponent|SetVelocity (Variables|Character|GetCharacterMovement) (Math|Vector|MakeVector (.x _returnvalue_2) (.y _returnvalue_2) (.z (Variables|/Script/Engine.MovementComponent|GetVelocity (Variables|Character|GetCharacterMovement))))))))))

(event Custom|CustomEvent
  ;[1 1 1] Dodge
  (if (and (> (Class|BaseCharacter|GetStamina) 0.0) (AI|Components|NavMovement|IsMovingonGround (Variables|Character|GetCharacterMovement)))
    (Utilities|FlowControl|DoOnce false
      (:Completed
        (GameplayEffects|ApplyGameplayEffectToSelf :self (Variables|Default|GetAbilitySystemComponent) :GameplayEffectClass "/Game/Blueprints/Character/Joyce/Ability/Effects/GE_Dodge.GE_Dodge_C")
        (Abilities|TryActivateAbilitiesbyTag (Variables|Default|GetAbilitySystemComponent) (Variables|GameplayTag|GetDodgeTagContainer) true)))))

(event Custom|ResetDodge
  ;[1 1 1] Dodge
  (Utilities|FlowControl|DoOnce false) ; enters at Reset
)

(event Custom|TriggerSword
  ;[1 1 1] Default Attack
  ;;[0 0 0] Trace On
  (bind _returnvalue (Utilities|Time|SetTimerbyEvent (delegate Custom|SwordLineTrace) 0.01 true))
  (Variables|Default|SetTriggerSwordEvent _returnvalue))

(event Custom|OnGuard
  (bind _charactermovement (Variables|Character|GetCharacterMovement))
  ;[1 1 1] Guard
  (if (not (or (AI|Components|NavMovement|IsFalling _charactermovement) (== (Variables|/Script/Engine.CharacterMovementComponent|GetMaxWalkSpeed _charactermovement) 9e+02)))
    (Variables|Default|SetIsBlocking true)
    (Variables|/Script/Engine.CharacterMovementComponent|SetMaxWalkSpeed (Variables|Character|GetCharacterMovement) 3e+02)
    (GameplayEffects|ApplyGameplayEffectToSelf :self (Variables|Default|GetAbilitySystemComponent) :GameplayEffectClass "/Game/Blueprints/Character/Joyce/Ability/Effects/GE_Guard.GE_Guard_C")
    (Development|SetHiddeninGame (Variables|Default|GetGuard) false false)))

(event Custom|StopTriggerSword
  ;[1 1 1] Default Attack
  ;;[0 0 0] Trace Off
  (Utilities|Time|ClearandInvalidateTimerbyHandle (Variables|Default|GetTriggerSwordEvent))
  (Utilities|FlowControl|DoOnce false) ; enters at Reset
)

(event Custom|Combo%20Attack
  (bind _mesh (Variables|Character|GetMesh))
  ;[1 1 1] Default Attack
  ;;[0 0 0] Combo
  (if (Variables|Default|GetIsAttackingCombo)
    (Variables|Default|SetIsBtnAttack true)
    (else
      (Variables|Default|SetIsAttackingCombo true)
      (if (>= (Class|BaseCharacter|GetStamina) 4.0)
        (GameplayEffects|ApplyGameplayEffectToSelf :self (Variables|Default|GetAbilitySystemComponent) :GameplayEffectClass "/Game/Blueprints/Character/Joyce/Ability/Effects/GE_AttackCost.GE_AttackCost_C")
        (switch int (Variables|Default|GetComboIndex)
          (:0
            (Variables|Default|SetComboIndex 1)
            (Variables|Default|SetComboMoveDistance 1.5e+02)
            (Animation|Montage|PlayMontage _mesh "/Game/Blueprints/Character/Joyce/Animation/Montage/AM_Combo1.AM_Combo1"
              (:then
                (Timeline|Timeline PlayFromStart
                  (:Update
                    (Variables|/Script/Engine.MovementComponent|SetVelocity (Variables|Character|GetCharacterMovement) (Math|Vector|MakeVector (.x (* (Transformation|GetActorForwardVector) (Variables|Default|GetComboMoveDistance))) (.y (* (Transformation|GetActorForwardVector) (Variables|Default|GetComboMoveDistance))) (.z (Variables|/Script/Engine.MovementComponent|GetVelocity (Variables|Character|GetCharacterMovement))))))))
              (:OnInterrupted
                (Utilities|FlowControl|RetriggerableDelay 0.8 :!label _label)
                (CallFunction|UpdateNotify))))
          (:1
            (Variables|Default|SetComboIndex 2)
            (Variables|Default|SetComboMoveDistance 1e+03)
            (Animation|Montage|PlayMontage _mesh "/Game/Blueprints/Character/Joyce/Animation/Montage/AM_Combo2.AM_Combo2"
              (:then
                (Timeline|Timeline PlayFromStart))
              (:OnInterrupted
                (goto _label))))
          (:2
            (Variables|Default|SetComboIndex 3)
            (Variables|Default|SetComboMoveDistance 0.0)
            (Animation|Montage|PlayMontage _mesh "/Game/Blueprints/Character/Joyce/Animation/Montage/AM_Combo3.AM_Combo3"
              (:then
                (Timeline|Timeline PlayFromStart))
              (:OnInterrupted
                (goto _label))))
          (:3
            (Variables|Default|SetComboIndex 0)
            (Variables|Default|SetComboMoveDistance 1e+03)
            (Animation|Montage|PlayMontage _mesh "/Game/Blueprints/Character/Joyce/Animation/Montage/AM_Combo4.AM_Combo4"
              (:then
                (Timeline|Timeline PlayFromStart))
              (:OnInterrupted
                (goto _label)))))
        (else
          (Variables|Default|SetIsAttackingCombo false))))))

(event Custom|OnSlash
  ;[1 1 1] Debug Key
  ;;[0 0 0] SlashSkill
  (Animation|Montage|PlayMontage (Variables|Character|GetMesh) "/Game/Blueprints/Character/Joyce/Animation/Montage/AM_JoyceSlashSkill.AM_JoyceSlashSkill"
    (:then
      (Input|DisableInput 0)
      (Utilities|FlowControl|Delay 2.0)
      (bind _returnvalue (Game|SpawnActorfromClass "/Game/Blueprints/Character/Joyce/Ability/BP_SlashSkill.BP_SlashSkill_C" (Math|Transform|MakeTransform (+ (Transformation|GetActorLocation) (* (Transformation|GetActorForwardVector) 2.5e+02)) "0, 0, 0" "1.000000,1.000000,1.000000") "AlwaysSpawn" self 0))
      (Input|EnableInput 0)
      (Utilities|FlowControl|Delay 2.0)
      (Actor|DestroyActor _returnvalue))))

(event Custom|OffGuard
  ;[1 1 1] Guard
  (Variables|Default|SetIsBlocking false)
  (Variables|/Script/Engine.CharacterMovementComponent|SetMaxWalkSpeed (Variables|Character|GetCharacterMovement) (Variables|Default|GetNormal%20Walk%20Speed))
  (GameplayEffects|RemoveActiveEffectswithTags (Variables|Default|GetAbilitySystemComponent) "(GameplayTags=((TagName=\"Ability.Guard\")))")
  (GameplayEffects|ApplyGameplayEffectToSelf :self (Variables|Default|GetAbilitySystemComponent) :GameplayEffectClass "/Game/Blueprints/Character/Joyce/Ability/Effects/GE_NoneGuard.GE_NoneGuard_C")
  (Development|SetHiddeninGame (Variables|Default|GetGuard) true false))

(event Custom|ServerScoreBall
  ;[1 1 1] Score
  (CallFunction|ScoreBall))

(event Input|EnhancedActionEvents|EnhancedInputActionIA_DefaultAttack
  (params (ActionValue :type Boolean) (ElapsedSeconds :type Float%20%28double-precision%29) (TriggeredSeconds :type Float%20%28double-precision%29) (InputAction :type Input%20Action%20Object%20Reference :default "/Game/Input/Action/IA_DefaultAttack.IA_DefaultAttack"))
  ;[1 1 1] Default Attack
  ;;[0 0 0] Attack Key Bind
  (:Triggered
    (if (and (AI|Components|NavMovement|IsMovingonGround (Variables|Character|GetCharacterMovement)) (not (Variables|Default|GetIsBlocking)))
      (Abilities|TryActivateAbilitiesbyTag (Variables|Default|GetAbilitySystemComponent) (Variables|GameplayTag|GetAttackTagContainer) true)
      (if (>= (Class|BaseCharacter|GetStamina) 4.0)
        (CallFunction|TriggerSword)))))

(event Input|EnhancedActionEvents|EnhancedInputActionIA_Dodge
  (params (ActionValue :type Boolean) (ElapsedSeconds :type Float%20%28double-precision%29) (TriggeredSeconds :type Float%20%28double-precision%29) (InputAction :type Input%20Action%20Object%20Reference :default "/Game/Input/Action/IA_Dodge.IA_Dodge"))
  ;[1 1 1] Dodge
  (:Triggered
    (CallFunction|CustomEvent))
  (:Completed
    (CallFunction|ResetDodge)))

(event Input|EnhancedActionEvents|EnhancedInputActionIA_Skill1
  (params (ActionValue :type Boolean) (ElapsedSeconds :type Float%20%28double-precision%29) (TriggeredSeconds :type Float%20%28double-precision%29) (InputAction :type Input%20Action%20Object%20Reference :default "/Game/Input/Action/IA_Skill1.IA_Skill1"))
  ;[1 1 1] Debug Key
  ;;[0 0 0] Thrust
  (:Triggered
    (if (AI|Components|NavMovement|IsMovingonGround (Variables|Character|GetCharacterMovement))
      (Abilities|TryActivateAbilitiesbyTag (Variables|Default|GetAbilitySystemComponent) (Variables|GameplayTag|GetSpiralTagContainer) true))))

(event Input|EnhancedActionEvents|EnhancedInputActionIA_Skill2
  (params (ActionValue :type Boolean) (ElapsedSeconds :type Float%20%28double-precision%29) (TriggeredSeconds :type Float%20%28double-precision%29) (InputAction :type Input%20Action%20Object%20Reference :default "/Game/Input/Action/IA_Skill2.IA_Skill2"))
  ;[1 1 1] Debug Key
  ;;[0 0 0] SlashSkill
  (:Triggered
    (if (AI|Components|NavMovement|IsMovingonGround (Variables|Character|GetCharacterMovement))
      (Abilities|TryActivateAbilitiesbyTag (Variables|Default|GetAbilitySystemComponent) (Variables|GameplayTag|GetSlashTagContainer) true))))

(event EventBeginPlay
  ;[1 1 1] Init
  (CallFunction|UpdateNotify))

(event EventOnDyingBP
  (bind _returnvalue (Pawn|GetController))
  (bind _asplayer_controller (Utilities|Casting|CastToPlayerController _returnvalue))
  ;[1 1 1] Die
  (CallFunction|ServerScoreBall)
  (CallFunction|ServerDeath)
  (CallFunction|ClientDeath)
  (Utilities|FlowControl|DoOnce false
    (:Completed
      (bind _returnvalue_2 (UserInterface|CreateWidget "/Game/Blueprints/UI/BP_WDG_Death.BP_WDG_Death_C" _asplayer_controller))
      (UserInterface|Viewport|AddtoViewport _returnvalue_2 0)
      (Input|SetInputModeUIOnly _asplayer_controller _returnvalue_2 "DoNotLock" true))))

(event EventTick
  (params (DeltaSeconds :type Float%20%28single-precision%29))
  ;[1 1 1] Tick
  (Utilities|FlowControl|Sequence
    (:then_0
      (CallFunction|CamShake)
      (Ability|Async|WaitGameplayEventToActor 0 "(TagName=\"Character.Damaged\")" true
        (:EventReceived
          (CallFunction|RPCAnyDamage))))
    (:then_1
      (Ability|Async|WaitGameplayEventToActor 0 "(TagName=\"Buff.Power\")" true
        (:EventReceived
          (CallFunction|PowerBuffRecv))))))

(event EventOnRespawn
  (bind _returnvalue (Pawn|GetController))
  (bind _asplayer_controller (Utilities|Casting|CastToPlayerController _returnvalue))
  ;[1 1 1] Die
  (Variables|Default|SetIsDead false)
  (Utilities|FlowControl|DoOnce false) ; enters at Reset
)

(event EventOnWin
  ;[1 1 1] WinLose
  (bind _returnvalue (UserInterface|CreateWidget "/Game/Blueprints/UI/WDG_Win.WDG_Win_C" (.AsPlayer%20Controller (Utilities|Casting|CastToPlayerController (Pawn|GetController)))))
  (UserInterface|Viewport|AddtoViewport _returnvalue 0))

(event EventOnLose
  ;[1 1 1] WinLose
  (bind _returnvalue (UserInterface|CreateWidget "/Game/Blueprints/UI/WDG_Lose.WDG_Lose_C" (.AsPlayer%20Controller (Utilities|Casting|CastToPlayerController (Pawn|GetController)))))
  (UserInterface|Viewport|AddtoViewport _returnvalue 0))

(event Input|KeyboardEvents|DebugKeyNumPadOne
  (params (Key :type Key%20Structure :default "None") (ActionValue :type Input%20Action%20Value%20Structure))
  ;[1 1 1] WinLose
  (:Pressed
    (bind _asbp_kid_king_player_state (Utilities|Casting|CastToBP_KidKingPlayerState (Variables|Default|GetPlayerState)))
    (Default|DebugAddScore _asbp_kid_king_player_state)))

(event Input|KeyboardEvents|Subtract
  (params (Key :type Key%20Structure :default "None"))
  ;[1 1 1] Debug Key
  ;;[0 0 0] Debug Hit
  (:Pressed
    (CallFunction|RPCDebugHit)))

(event Input|MouseEvents|RightMouseButton
  (params (Key :type Key%20Structure :default "None"))
  ;[1 1 1] Guard
  (:Pressed
    (CallFunction|OnGuardServer))
  (:Released
    (CallFunction|OffGuardSever)))

(event Input|KeyboardEvents|Equals
  (params (Key :type Key%20Structure :default "None"))
  ;[1 1 1] Debug Key
  ;;[0 0 0] Give Buff
  (:Pressed
    (GameplayEffects|ApplyGameplayEffectToSelf :self (Variables|Default|GetAbilitySystemComponent) :GameplayEffectClass "/Game/Blueprints/Character/Joyce/Ability/Effects/GE_PowerUp.GE_PowerUp_C")
    (bind _returnvalue (Niagara|SpawnSystemAttached "/Game/resource/Buff_NS/STRBuff_NS.STRBuff_NS" (Variables|Character|GetMesh) "None" "0, 0, 0" "0, 0, 0" "KeepRelativeOffset" false))
    (Utilities|FlowControl|Delay (Variables|Default|GetBuffDuration))
    (GameplayEffects|RemoveActiveEffectswithTags (Variables|Default|GetAbilitySystemComponent) "(GameplayTags=((TagName=\"Test.Buff\")))")
    (Components|DestroyComponent _returnvalue)))

(event Input|KeyboardEvents|Multiply
  (params (Key :type Key%20Structure :default "None"))
  ;[1 1 1] Debug Key
  ;;[0 0 0] Print Health & Stamina
  (:Pressed
    (Development|PrintString (Utilities|String|Append "Health: " (Utilities|String|ToString(Float) (Class|BaseCharacter|GetHealth))))
    (Development|PrintString (Utilities|String|Append "Stamina: " (Utilities|String|ToString(Float) (Class|BaseCharacter|GetStamina))))))

(event Input|KeyboardEvents|NumPadOne
  (params (Key :type Key%20Structure :default "None"))
  (:Pressed
    (CallFunction|IncreaseTime)))

(fn ConstructionScript)

(fn HitCamShake
  (Camera|PlayWorldCameraShake "/Game/Blueprints/CamShake/HitCamShake_BP.HitCamShake_BP_C" (Transformation|GetActorLocation) 0.0 1e+03))

(fn GetCooldownPercentbyTag
  (params (Tags :type Gameplay%20Tag%20Container%20Structure))
  (bind _returnvalue (GameplayEffects|GetActiveEffectswithAllTags (Variables|Default|GetAbilitySystemComponent) Tags))
  (if (Utilities|Array|IsNotEmpty _returnvalue)
    (for _array_element _returnvalue
      (bind _returnvalue_2 (Ability|GameplayEffect|GetActiveGameplayEffectRemainingDuration _array_element))
      (return (/ _returnvalue_2 5.0)))))