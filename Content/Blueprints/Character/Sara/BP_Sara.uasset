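; Sara player character built on GAS, with combo attack, dodge, WaterBall and LightningSphere skills, and a guard.
; Input mostly activates abilities by tag; action events play montages and spawn delayed attack actors, while gameplay effects handle stamina, guard and buffs.
; Tick drives speed-based camera shake and creates damage and power-buff event listeners.
; Death spawns score balls and opens a death widget; win/lose widgets and debug keys are included.
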(event Custom|RPC_AnyDamage
  ;[1 1 1] Damaged
  (if (> (Class|BaseCharacter|GetHealth) 0.0)
    (Animation|PlayAnimMontage "/Game/Blueprints/Character/Sara/Animation/Montage/AM_SaraHit.AM_SaraHit" 1.0 "None")))

(event Custom|CamShake
  (bind _returnvalue (Pawn|GetController))
  (bind _as플레이어_컨트롤러 (Utilities|Casting|CastToPlayerController _returnvalue))
  ;[1 1 1] CamShake
  (if (<= (Math|Vector|VectorLength (Transformation|GetVelocity)) 0.0)
    (Game|Feedback|ClientStartCameraShake _as플레이어_컨트롤러 "/Game/Blueprints/CamShake/IdleCamShake_BP.IdleCamShake_BP_C" 1.0 "CameraLocal" "0, 0, 0")
    (elif (>= (Math|Vector|VectorLength (Transformation|GetVelocity)) 301.0)
      (Game|Feedback|ClientStartCameraShake _as플레이어_컨트롤러 "/Game/Blueprints/CamShake/RunCamShake_BP.RunCamShake_BP_C" 1.0 "CameraLocal" "0, 0, 0")
      (else
        (Game|Feedback|ClientStartCameraShake _as플레이어_컨트롤러 "/Game/Blueprints/CamShake/WalkCamShake_BP.WalkCamShake_BP_C" 1.0 "CameraLocal" "0, 0, 0")))))

(event Custom|Btn%20Attack
  (bind _mesh (Variables|Character|GetMesh))
  ;[1 1 1] DefaultAttack
  ;;[0 0 0] Combo
  (if (Variables|Default|GetIsBtnAttack)
    (Variables|Default|SetIsBtnAttack false)
    (if (>= (Class|BaseCharacter|GetStamina) 4.0)
      (GameplayEffects|ApplyGameplayEffectToSelf :self (Variables|Default|GetAbilitySystemComponent) :GameplayEffectClass "/Game/Blueprints/Character/Joyce/Ability/Effects/GE_AttackCost.GE_AttackCost_C")
      (switch int (Variables|Default|GetComboIndex)
        (:0
          (Variables|Default|SetComboIndex 1)
          (Variables|Default|SetComboMoveDistance 0.0)
          (Animation|Montage|PlayMontage _mesh "/Game/Blueprints/Character/Sara/Animation/Montage/AM_SaraCombo1.AM_SaraCombo1"
            (:then
              (Utilities|FlowControl|Delay 0.5 :!label _label)
              (Game|SpawnActorfromClass "/Game/Blueprints/Character/Sara/Skill/BP_DefaultAttack.BP_DefaultAttack_C" (Transformation|GetWorldTransform (Variables|Default|GetScene)) "AlwaysSpawn" self 1.5e+03 0.0 0))
            (:OnInterrupted
              (Utilities|FlowControl|RetriggerableDelay 0.8 :!label _label_2)
              (CallFunction|NotifyReset))))
        (:1
          (Variables|Default|SetComboIndex 2)
          (Variables|Default|SetComboMoveDistance 0.0)
          (Animation|Montage|PlayMontage _mesh "/Game/Blueprints/Character/Sara/Animation/Montage/AM_SaraCombo2.AM_SaraCombo2"
            (:then
              (goto _label))
            (:OnInterrupted
              (goto _label_2))))
        (:2
          (Variables|Default|SetComboIndex 0)
          (Variables|Default|SetComboMoveDistance 0.0)
          (Animation|Montage|PlayMontage _mesh "/Game/Blueprints/Character/Sara/Animation/Montage/AM_SaraCombo3.AM_SaraCombo3"
            (:then
              (Utilities|FlowControl|Delay 0.5)
              (Game|SpawnActorfromClass "/Game/Blueprints/Character/Sara/Skill/BP_DefaultAttack.BP_DefaultAttack_C" (Transformation|GetWorldTransform (Variables|Default|GetScene1)) "AlwaysSpawn" self 1.5e+03 4.0 0)
              (Utilities|FlowControl|Delay 0.5))
            (:OnInterrupted
              (goto _label_2)))))
      (else
        (Variables|Default|SetIsAttackingCombo false)
        (Variables|Default|SetIsBtnAttack false)))))

(event Custom|OnGuardServer
  ;[1 1 1] Guard
  (CallFunction|OnGuard))

(event Custom|OffGuardSever
  ;[1 1 1] Guard
  (CallFunction|OffGuard))

(event Custom|IncreaseTime
  (bind _asbp_game_state (Utilities|Casting|CastToBP_GameState (Game|GetGameState)))
  (Default|IncreaseTime _asbp_game_state))

(event Custom|Client%20Death
  ;[1 1 1] Die
  (Variables|Default|SetIsDead true))

(event Custom|ResetCombo
  ;[1 1 1] DefaultAttack
  ;;[0 0 0] Combo
  (Variables|Default|SetIsAttackingCombo false)
  (Variables|Default|SetIsBtnAttack false)
  (Variables|Default|SetComboIndex 0))

(event Custom|ScoreBall
  ;[1 1 1] Score
  (if (not (== (Variables|Default|GetScoreIndex) 5)) :!label _label
    (Utilities|FlowControl|Delay 0.2)
    (Game|SpawnActorfromClass "/Game/Blueprints/Score/BP_ScoreBall.BP_ScoreBall_C" (Math|Transform|MakeTransform (.location (Transformation|GetWorldTransform (Variables|Default|GetScene))) (Math|Rotator|MakeRotator 0.0 0.0 (.yaw (Math|Random|RandomRotator false))) "1.000000,1.000000,1.000000") "Undefined" 0 3e+02 0.5 0)
    (Variables|Default|SetScoreIndex (+ (Variables|Default|GetScoreIndex) 1))
    (goto _label)))

(event Custom|NotifyReset
  (Input|EnableInput 0)
  (CallFunction|ResetCombo))

(event Custom|Server%20Death
  ;[1 1 1] Die
  (Variables|Default|SetIsDead true))

(event Custom|Dodge
  (bind _returnvalue (Transformation|GetActorForwardVector))
  (bind _dodgedistance (Variables|Default|GetDodgeDistance))
  (bind _returnvalue_2 (* _returnvalue _dodgedistance))
  ;[1 1 1] Dodge
  (Animation|Montage|PlayMontage (Variables|Character|GetMesh) "/Game/Blueprints/Character/Sara/Animation/Montage/AM_DashMontage.AM_DashMontage"
    (:then
      ;;[1 1 1] Don't Used
      (Timeline|타임라인_0 PlayFromStart
        (:Update
          (Variables|/Script/Engine.MovementComponent|SetVelocity (Variables|Character|GetCharacterMovement) (Math|Vector|MakeVector (.x _returnvalue_2) (.y _returnvalue_2) (.z (Variables|/Script/Engine.MovementComponent|GetVelocity (Variables|Character|GetCharacterMovement))))))))))

(event Custom|PowerBuffRecv
  ;[1 1 1] Powerup Buff
  (CallFunction|PowerBuffRecvREP))

(event Custom|PowerBuffRecv_REP
  ;[1 1 1] Powerup Buff
  (GameplayEffects|ApplyGameplayEffectToSelf :self (Variables|Default|GetAbilitySystemComponent) :GameplayEffectClass "/Game/Blueprints/Character/Joyce/Ability/Effects/GE_PowerUp.GE_PowerUp_C")
  (Utilities|FlowControl|DoOnce false :!label _label
    (:Completed
      (bind _returnvalue (Niagara|SpawnSystemAttached "/Game/resource/Buff_NS/SaraSTRBuff_NS.SaraSTRBuff_NS" (Variables|Character|GetMesh) "None" "0, 0, 0" "0, 0, 0" "KeepRelativeOffset" false))
      (Utilities|FlowControl|Delay (Variables|Default|GetBuffDuration))
      (GameplayEffects|RemoveActiveEffectswithTags (Variables|Default|GetAbilitySystemComponent) "(GameplayTags=((TagName=\"Test.Buff\")))")
      (Components|DestroyComponent _returnvalue)
      (goto _label Reset))))

(event Custom|WaterBall
  ;[1 1 1] Skill
  ;;[0 0 0] WaterBall
  (Animation|Montage|PlayMontage (Variables|Character|GetMesh) "/Game/Blueprints/Character/Sara/Animation/Montage/AM_SaraWaterBall.AM_SaraWaterBall"
    (:then
      (Utilities|FlowControl|Delay 1.7)
      (Game|SpawnActorfromClass "/Game/Blueprints/Character/Sara/Skill/BP_WaterBall.BP_WaterBall_C" (Transformation|GetWorldTransform (Variables|Default|GetScene)) "AlwaysSpawn" self 1.5e+03 0.0 0))))

(event Custom|OnGuard
  (bind _charactermovement (Variables|Character|GetCharacterMovement))
  ;[1 1 1] Guard
  (if (not (or (AI|Components|NavMovement|IsFalling _charactermovement) (== (Variables|/Script/Engine.CharacterMovementComponent|GetMaxWalkSpeed _charactermovement) 9e+02)))
    (Variables|Default|SetIsBlocking true)
    (Variables|/Script/Engine.CharacterMovementComponent|SetMaxWalkSpeed (Variables|Character|GetCharacterMovement) 3e+02)
    (GameplayEffects|ApplyGameplayEffectToSelf :self (Variables|Default|GetAbilitySystemComponent) :GameplayEffectClass "/Game/Blueprints/Character/Joyce/Ability/Effects/GE_Guard.GE_Guard_C")
    (Development|SetHiddeninGame (Variables|Default|GetGuard) false false)))

(event Custom|Lightening%20Sphere
  (bind _scene3 (Variables|Default|GetScene3))
  (bind _returnvalue (Transformation|GetWorldTransform _scene3))
  ;[1 1 1] Skill
  ;;[0 0 0] Lightning Sphere
  (Animation|Montage|PlayMontage (Variables|Character|GetMesh) "/Game/Blueprints/Character/Sara/Animation/Montage/AM_SaraLightningSphere.AM_SaraLightningSphere"
    (:then
      (Utilities|FlowControl|Delay 2.0)
      (Niagara|SpawnSystematLocation "/Game/resource/Actors/MainCharacter/SaraSkill/LightningSphere/LightningSpawner.LightningSpawner" (.location _returnvalue) (.rotation _returnvalue) (.scale _returnvalue))
      (Utilities|FlowControl|Delay 2.0)
      (bind _returnvalue_2 (Game|SpawnActorfromClass "/Game/Blueprints/Character/Sara/Skill/LightningSkill.LightningSkill_C" (Transformation|GetWorldTransform (Variables|Default|GetScene2)) "AlwaysSpawn" self 0))
      (Utilities|FlowControl|Delay 5.0)
      (Actor|DestroyActor _returnvalue_2))))

(event Custom|Combo%20Attack
  (bind _mesh (Variables|Character|GetMesh))
  ;[1 1 1] DefaultAttack
  ;;[0 0 0] Combo
  (if (Variables|Default|GetIsAttackingCombo)
    (Variables|Default|SetIsBtnAttack true)
    (else
      (Variables|Default|SetIsAttackingCombo true)
      (if (>= (Class|BaseCharacter|GetStamina) 4.0)
        (GameplayEffects|ApplyGameplayEffectToSelf :self (Variables|Default|GetAbilitySystemComponent) :GameplayEffectClass "/Game/Blueprints/Character/Joyce/Ability/Effects/GE_AttackCost.GE_AttackCost_C")
        (switch int (Variables|Default|GetComboIndex)
          (:0
            (Variables|Default|SetComboIndex 1)
            (Variables|Default|SetComboMoveDistance 0.0)
            (Animation|Montage|PlayMontage _mesh "/Game/Blueprints/Character/Sara/Animation/Montage/AM_SaraCombo1.AM_SaraCombo1"
              (:then
                (Utilities|FlowControl|Delay 0.5 :!label _label)
                (Game|SpawnActorfromClass "/Game/Blueprints/Character/Sara/Skill/BP_DefaultAttack.BP_DefaultAttack_C" (Transformation|GetWorldTransform (Variables|Default|GetScene)) "AlwaysSpawn" self 1.5e+03 0.0 0))
              (:OnInterrupted
                (Utilities|FlowControl|RetriggerableDelay 0.8 :!label _label_2)
                (CallFunction|NotifyReset))))
          (:1
            (Variables|Default|SetComboIndex 2)
            (Variables|Default|SetComboMoveDistance 0.0)
            (Animation|Montage|PlayMontage _mesh "/Game/Blueprints/Character/Sara/Animation/Montage/AM_SaraCombo2.AM_SaraCombo2"
              (:then
                (goto _label))
              (:OnInterrupted
                (goto _label_2))))
          (:2
            (Variables|Default|SetComboIndex 0)
            (Variables|Default|SetComboMoveDistance 0.0)
            (Animation|Montage|PlayMontage _mesh "/Game/Blueprints/Character/Sara/Animation/Montage/AM_SaraCombo3.AM_SaraCombo3"
              (:then
                (Utilities|FlowControl|Delay 0.5)
                (Game|SpawnActorfromClass "/Game/Blueprints/Character/Sara/Skill/BP_DefaultAttack.BP_DefaultAttack_C" (Transformation|GetWorldTransform (Variables|Default|GetScene1)) "AlwaysSpawn" self 1.5e+03 4.0 0)
                (Utilities|FlowControl|Delay 0.5))
              (:OnInterrupted
                (goto _label_2)))))
        (else
          (Variables|Default|SetIsAttackingCombo false)
          (Variables|Default|SetIsBtnAttack false))))))

(event Custom|RPC%20Debug%20Hit
  (GameplayEffects|ApplyGameplayEffectToSelf :self (Variables|Default|GetAbilitySystemComponent) :GameplayEffectClass "/Game/Blueprints/Character/Joyce/Ability/Effects/GE_DamageSample.GE_DamageSample_C")
  (Ability|SendGameplayEventtoActor self "(TagName=\"Character.Damaged\")" (Utilities|Struct|MakeGameplayEventData "(TagName=\"Character.Damaged\")" self)))

(event Custom|OffGuard
  ;[1 1 1] Guard
  (Variables|Default|SetIsBlocking false)
  (Variables|/Script/Engine.CharacterMovementComponent|SetMaxWalkSpeed (Variables|Character|GetCharacterMovement) 8e+02)
  (GameplayEffects|RemoveActiveEffectswithTags (Variables|Default|GetAbilitySystemComponent) "(GameplayTags=((TagName=\"Ability.Guard\")))")
  (GameplayEffects|ApplyGameplayEffectToSelf :self (Variables|Default|GetAbilitySystemComponent) :GameplayEffectClass "/Game/Blueprints/Character/Joyce/Ability/Effects/GE_NoneGuard.GE_NoneGuard_C")
  (Development|SetHiddeninGame (Variables|Default|GetGuard) true false))

(event Custom|ServerScoreBall
  ;[1 1 1] Score
  (CallFunction|ScoreBall))

(event Input|EnhancedActionEvents|EnhancedInputActionIA_DefaultAttack
  (params (ActionValue :type Boolean) (ElapsedSeconds :type Float%20%28double-precision%29) (TriggeredSeconds :type Float%20%28double-precision%29) (InputAction :type Input%20Action%20Object%20Reference :default "/Game/Input/Action/IA_DefaultAttack.IA_DefaultAttack"))
  ;[1 1 1] DefaultAttack
  (:Triggered
    (if (AI|Components|NavMovement|IsMovingonGround (Variables|Character|GetCharacterMovement))
      (Abilities|TryActivateAbilitiesbyTag (Variables|Default|GetAbilitySystemComponent) (Variables|GamePlayTag|GetComboAttack%20Tag%20Container) true))))

(event Input|EnhancedActionEvents|EnhancedInputActionIA_Dodge
  (params (ActionValue :type Boolean) (ElapsedSeconds :type Float%20%28double-precision%29) (TriggeredSeconds :type Float%20%28double-precision%29) (InputAction :type Input%20Action%20Object%20Reference :default "/Game/Input/Action/IA_Dodge.IA_Dodge"))
  ;[1 1 1] Dodge
  (:Triggered
    (if (and (> (Class|BaseCharacter|GetStamina) 0.0) (AI|Components|NavMovement|IsMovingonGround (Variables|Character|GetCharacterMovement)))
      (Utilities|FlowControl|DoOnce false :!label _label
        (:Completed
          (GameplayEffects|ApplyGameplayEffectToSelf :self (Variables|Default|GetAbilitySystemComponent) :GameplayEffectClass "/Game/Blueprints/Character/Joyce/Ability/Effects/GE_Dodge.GE_Dodge_C")
          (Abilities|TryActivateAbilitiesbyTag (Variables|Default|GetAbilitySystemComponent) (Variables|GamePlayTag|GetDodge%20Tag%20Container) true)))))
  (:Completed
    (goto _label Reset)))

(event Input|EnhancedActionEvents|EnhancedInputActionIA_Skill2
  (params (ActionValue :type Boolean) (ElapsedSeconds :type Float%20%28double-precision%29) (TriggeredSeconds :type Float%20%28double-precision%29) (InputAction :type Input%20Action%20Object%20Reference :default "/Game/Input/Action/IA_Skill2.IA_Skill2"))
  ;[1 1 1] Skill
  ;;[0 0 0] Lightning Sphere
  (:Triggered
    (if (AI|Components|NavMovement|IsMovingonGround (Variables|Character|GetCharacterMovement))
      (Abilities|TryActivateAbilitiesbyTag (Variables|Default|GetAbilitySystemComponent) (Variables|GamePlayTag|GetLightningSphere%20Tag%20Container) true))))

(event Input|EnhancedActionEvents|EnhancedInputActionIA_Skill1
  (params (ActionValue :type Boolean) (ElapsedSeconds :type Float%20%28double-precision%29) (TriggeredSeconds :type Float%20%28double-precision%29) (InputAction :type Input%20Action%20Object%20Reference :default "/Game/Input/Action/IA_Skill1.IA_Skill1"))
  ;[1 1 1] Skill
  ;;[0 0 0] WaterBall
  (:Triggered
    (if (AI|Components|NavMovement|IsMovingonGround (Variables|Character|GetCharacterMovement))
      (Abilities|TryActivateAbilitiesbyTag (Variables|Default|GetAbilitySystemComponent) (Variables|GamePlayTag|GetWaterBall%20Tag%20Container) true))))

(event EventBeginPlay)

(event EventOnDyingBP
  (bind _returnvalue (Pawn|GetController))
  (bind _as플레이어_컨트롤러 (Utilities|Casting|CastToPlayerController _returnvalue))
  ;[1 1 1] Die
  (CallFunction|ServerScoreBall)
  (CallFunction|ServerDeath)
  (CallFunction|ClientDeath)
  (Utilities|FlowControl|DoOnce false
    (:Completed
      (bind _returnvalue_2 (UserInterface|CreateWidget "/Game/Blueprints/UI/BP_WDG_Death.BP_WDG_Death_C" _as플레이어_컨트롤러))
      (UserInterface|Viewport|AddtoViewport _returnvalue_2 0)
      (Input|SetInputModeUIOnly _as플레이어_컨트롤러 _returnvalue_2 "DoNotLock" true))))

(event EventTick
  (params (DeltaSeconds :type Float%20%28single-precision%29))
  ;[1 1 1] Tick
  (Utilities|FlowControl|Sequence
    (:then_0
      (CallFunction|CamShake)
      (Ability|Async|WaitGameplayEventToActor 0 "(TagName=\"Character.Damaged\")" true
        (:EventReceived
          (CallFunction|RPCAnyDamage))))
    (:then_1
      (Ability|Async|WaitGameplayEventToActor 0 "(TagName=\"Buff.Power\")" true
        (:EventReceived
          (CallFunction|PowerBuffRecv))))))

(event EventOnRespawn
  (bind _returnvalue (Pawn|GetController))
  (bind _as플레이어_컨트롤러 (Utilities|Casting|CastToPlayerController _returnvalue))
  ;[1 1 1] Die
  (Variables|Default|SetIsDead false)
  (Utilities|FlowControl|DoOnce false) ; enters at Reset
)

(event EventOnWin
  ;[1 1 1] WinLose
  (bind _returnvalue (UserInterface|CreateWidget "/Game/Blueprints/UI/WDG_Win.WDG_Win_C" (.As플레이어%20컨트롤러 (Utilities|Casting|CastToPlayerController (Pawn|GetController)))))
  (UserInterface|Viewport|AddtoViewport _returnvalue 0))

(event EventOnLose
  ;[1 1 1] WinLose
  (bind _returnvalue (UserInterface|CreateWidget "/Game/Blueprints/UI/WDG_Lose.WDG_Lose_C" (.As플레이어%20컨트롤러 (Utilities|Casting|CastToPlayerController (Pawn|GetController)))))
  (UserInterface|Viewport|AddtoViewport _returnvalue 0))

(event Collision|EventActorBeginOverlap
  (params (OtherActor :type Actor%20Object%20Reference)))

(event Input|KeyboardEvents|Subtract
  (params (Key :type Key%20Structure :default "None"))
  (:Pressed
    (CallFunction|RPCDebugHit)))

(event Input|MouseEvents|RightMouseButton
  (params (Key :type Key%20Structure :default "None"))
  ;[1 1 1] Guard
  (:Pressed
    (CallFunction|OnGuardServer))
  (:Released
    (CallFunction|OffGuardSever)))

(event Input|KeyboardEvents|Add
  (params (Key :type Key%20Structure :default "None"))
  ;[1 1 1] WinLose
  (:Pressed
    (bind _asbp_kid_king_player_state (Utilities|Casting|CastToBP_KidKingPlayerState (Variables|Default|GetPlayerState)))
    (Default|DebugAddScore _asbp_kid_king_player_state)))

(event Input|KeyboardEvents|NumPadOne
  (params (Key :type Key%20Structure :default "None"))
  (:Pressed
    (CallFunction|IncreaseTime)))

(fn ConstructionScript)

(fn HitCamShake
  (Camera|PlayWorldCameraShake "/Game/Blueprints/CamShake/HitCamShake_BP.HitCamShake_BP_C" (Transformation|GetActorLocation) 0.0 1e+03))

(fn GetCooldownPercentbyTag
  (params (Tags :type Gameplay%20Tag%20Container%20Structure))
  (bind _returnvalue (GameplayEffects|GetActiveEffectswithAllTags (Variables|Default|GetAbilitySystemComponent) Tags))
  (if (Utilities|Array|IsNotEmpty _returnvalue)
    (for _array_element _returnvalue
      (bind _returnvalue_2 (Ability|GameplayEffect|GetActiveGameplayEffectRemainingDuration _array_element))
      (return (/ _returnvalue_2 5.0)))))