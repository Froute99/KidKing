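; BP_DefaultAttack is the actor for Sara's default attack, dealing damage through the Gameplay Ability System when it hits something.
; On the first hit against an actor with an ability system component, that component applies GE_DamageSample to itself.
; It then sends a Character.Damaged gameplay event to the victim, with the attack as instigator.
; A DoOnce limits each attack instance to one damage application.
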(event Custom|OnActorHit_Event
  (params (SelfActor :type Actor%20Object%20Reference) (OtherActor :type Actor%20Object%20Reference) (NormalImpulse :type Vector) (Hit :type Hit%20Result%20Structure%20%28by%20ref%29))
  (bind _returnvalue (Ability|GetAbilitySystemComponent OtherActor))
  (Utilities|IsValid _returnvalue
    (:Is%20Valid
      (Utilities|FlowControl|DoOnce false
        (:Completed
          (GameplayEffects|ApplyGameplayEffectToTarget :self _returnvalue :GameplayEffectClass "/Game/Blueprints/Character/Joyce/Ability/Effects/GE_DamageSample.GE_DamageSample_C" :Target _returnvalue)
          (Ability|SendGameplayEventtoActor OtherActor "(TagName=\"Character.Damaged\")" (Utilities|Struct|MakeGameplayEventData "(TagName=\"\")" self OtherActor 0 0 "()" "(GameplayTags=)" "(GameplayTags=)" 0.0 (Ability|TargetData|AbilityTargetDatafromActor OtherActor))))))))

(event EventBeginPlay
  (|CallParentFunction)
  (Collision|AssignOnActorHit (delegate Custom|OnActorHit_Event)))

(event Collision|EventActorBeginOverlap
  (params (OtherActor :type Actor%20Object%20Reference))
  (|CallParentFunction OtherActor) ; 지금 이 노드는 비활성 상태입니다. \n핀을 끌어서 다른 노드를 연결하면 활성화됩니다.
)

(event EventTick
  (params (DeltaSeconds :type Float%20%28single-precision%29))
  (|CallParentFunction DeltaSeconds) ; 지금 이 노드는 비활성 상태입니다. \n핀을 끌어서 다른 노드를 연결하면 활성화됩니다.
)

(fn ConstructionScript
  (|CallParentFunction))