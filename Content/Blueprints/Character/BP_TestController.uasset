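; Player controller that handles character selection and spawning, apparently for testing given its name.
; On post-login it shows the character selection widget, and its spawn RPC event has BP_KidKingGameMode spawn the chosen character at Player1Start with the controller's team, then possesses it.
; Thrust cooldown progress is forwarded to the player HUD.
; Slash cooldown is an empty stub, and some unconnected debug and golem-targeting nodes remain.
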(event Custom|RPC_SpawnPlayer
  (params (Character%20Index :type Integer))
  ;[0 0 0] Spawn Player
  (Variables|Default|SetCharacter%20Index Character%20Index)
  (if (Pawn|IsLocalPlayerController)
    _
    (else
      _))
  (bind _asbp_kid_king_game_mode (Utilities|Casting|CastToBP_KidKingGameMode (Game|GetGameMode)))
  (bind _returnvalue (Default|SpawnPlayer _asbp_kid_king_game_mode self "Player1Start" (Variables|Default|GetCharacter%20Index) (Variables|Default|GetTeamIndex)))
  (Pawn|Possess self _returnvalue))

(event Custom|ThrustCooldown
  (params (Current%20Percent :type Float%20%28double-precision%29))
  (Default|SetCooldown (Variables|Default|GetREF%20PlayerHUD) Current%20Percent))

(event Custom|OnPostLogin
  ;[0 0 0] Spawn Player
  (bind _returnvalue (UserInterface|CreateWidget "/Game/Blueprints/UI/BP_WDG_CharacterSelection.BP_WDG_CharacterSelection_C" self))
  (UserInterface|Viewport|AddtoPlayerScreen _returnvalue))

(event Custom|SlashCooldown)

(event EventBeginPlay
  ;[0 0 0] Spawn Player
)

(fn ConstructionScript)