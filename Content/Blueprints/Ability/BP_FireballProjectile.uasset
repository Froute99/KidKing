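; Fireball projectile Blueprint for an ability, which destroys itself on overlap or hit.
; On Hit, it applies fixed damage to the struck actor with the instigator as damage causer, prints the result, then destroys itself.
; On actor overlap, it destroys itself and prints the other actor's name without applying damage.
; An owner-filter check exists but is disconnected, so overlaps are not filtered.
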(event Collision|EventActorBeginOverlap
  (params (OtherActor :type Actor%20Object%20Reference))
  (Actor|DestroyActor)
  (Development|PrintString (Utilities|GetDisplayName OtherActor)))

(event Collision|EventHit
  (params (MyComp :type Primitive%20Component%20Object%20Reference) (Other :type Actor%20Object%20Reference) (OtherComp :type Primitive%20Component%20Object%20Reference) (bSelfMoved :type Boolean) (HitLocation :type Vector :default "0, 0, 0") (HitNormal :type Vector :default "0, 0, 0") (NormalImpulse :type Vector :default "0, 0, 0") (Hit :type Hit%20Result%20Structure%20%28by%20ref%29))
  (bind _returnvalue (Game|Damage|ApplyDamage Other 5e+01 0 (Game|GetInstigator) "/Script/Engine.DamageType"))
  (Development|PrintString (Utilities|String|ToString(Float) _returnvalue))
  (Actor|DestroyActor))

(fn ConstructionScript)