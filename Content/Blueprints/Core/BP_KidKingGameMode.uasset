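; Game mode for Kid King that runs a timed, score-based match and manages its players and AI bots.
; Tick polls the game state clock to spawn a Golem early, swap it for an Elder midway and track the top player score.
; At ten minutes it pauses the game and calls Win or Lose on each pawn.
; SpawnPlayer replaces a controller's pawn with the selected character at a random PlayerStart.
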(event Custom|spawnGolem
  (bind _ref_gamestate (Variables|REF|GetREF%20GameState))
  ;[1 1 1] SpawnBot
  (if (and (>= (Variables|/Game/Blueprints/Core/BP_GameState.BP_GameState_C|GetMinutes _ref_gamestate) 0) (>= (Variables|/Game/Blueprints/Core/BP_GameState.BP_GameState_C|GetSeconds _ref_gamestate) 15))
    (Utilities|FlowControl|DoOnce false
      (:Completed
        (bind _returnvalue (AI|SpawnAIFromClass "/Game/Blueprints/Bot/Golem/BP_Golem.BP_Golem_C" "/Game/Blueprints/Bot/Golem/BT_Golem.BT_Golem" (Transformation|GetActorLocation (Variables|REF|GetSpawner%20REF)) "0, 0, 0" false 0))
        (Variables|Default|SetGolem _returnvalue)))))

(event Custom|ElderSpawn
  ;[1 1 1] SpawnBot
  (if (>= (Variables|/Game/Blueprints/Core/BP_GameState.BP_GameState_C|GetMinutes (Variables|REF|GetREF%20GameState)) 5)
    (Utilities|FlowControl|DoOnce false
      (:Completed
        (Actor|DestroyActor (Variables|Default|GetGolem))
        (AI|SpawnAIFromClass "/Game/Blueprints/Bot/Elder/BP_Elder.BP_Elder_C" "/Game/Blueprints/Bot/Elder/BT_Elder.BT_Elder" (Transformation|GetActorLocation (Variables|REF|GetSpawner%20REF)) "0, 0, 0" false 0)))))

(event Custom|JudgementSystem
  (if (== (Variables|/Game/Blueprints/Core/BP_GameState.BP_GameState_C|GetMinutes (Variables|REF|GetREF%20GameState)) 10)
    (Game|SetGamePaused true)
    (for _array_element (Variables|REF|GetPCs)
      (if (== (Variables|Default|GetMaximumScore) (Variables|/Game/Blueprints/Character/BP_KidKingPlayerState.BP_KidKingPlayerState_C|GetPlayerScore (.AsBP%20Kid%20King%20Player%20State (Utilities|Casting|CastToBP_KidKingPlayerState (Variables|/Script/Engine.Controller|GetPlayerState _array_element)))))
        (bind _asbase_character (Utilities|Casting|CastToBaseCharacter (Pawn|GetControlledPawn _array_element)))
        (Class|BaseCharacter|Win _asbase_character)
        (else
          (bind _asbase_character_2 (Utilities|Casting|CastToBaseCharacter (Pawn|GetControlledPawn _array_element)))
          (Class|BaseCharacter|Lose _asbase_character_2))))))

(event Custom|Get%20MaximumScore
  (for _array_element (Variables|REF|GetPCs)
    (bind _asbp_kid_king_player_state (Utilities|Casting|CastToBP_KidKingPlayerState (Variables|/Script/Engine.Controller|GetPlayerState _array_element)))
    (if (>= (Variables|/Game/Blueprints/Character/BP_KidKingPlayerState.BP_KidKingPlayerState_C|GetPlayerScore _asbp_kid_king_player_state) (Variables|Default|GetMaximumScore))
      (Variables|Default|SetMaximumScore (Variables|/Game/Blueprints/Character/BP_KidKingPlayerState.BP_KidKingPlayerState_C|GetPlayerScore _asbp_kid_king_player_state)))))

(event EventPostLogin
  (params (NewPlayer :type Player%20Controller%20Object%20Reference))
  (Utilities|Array|Add (Variables|REF|GetPCs) NewPlayer)
  (Development|PrintString (Utilities|String|Append "Hi," (Utilities|GetDisplayName NewPlayer)))
  (bind _asbp_test_controller (Utilities|Casting|CastToBP_TestController NewPlayer)
    (:then
      (Default|OnPostLogin _asbp_test_controller))
    (:CastFailed
      (Development|PrintString "Cast Failed in KidKingGameMode"))))

(event EventBeginPlay
  (Utilities|FlowControl|Sequence
    (:then_0
      (bind _outactors (Actor|GetAllActorsOfClass "/Game/Blueprints/Bot/Spawner/Bot_Spawner.Bot_Spawner_C"))
      (Variables|REF|SetSpawner%20REF (Utilities|Array|Get(acopy) _outactors)))
    (:then_1
      (bind _outactors_2 (Actor|GetAllActorsOfClass "/Game/Blueprints/Core/BP_GameState.BP_GameState_C"))
      (Variables|REF|SetREF%20GameState (Utilities|Array|Get(acopy) _outactors_2)))))

(event EventTick
  (params (DeltaSeconds :type Float%20%28single-precision%29))
  (Utilities|FlowControl|Sequence
    (:then_1
      (CallFunction|SpawnGolem))
    (:then_2
      (CallFunction|ElderSpawn))
    (:then_3
      (CallFunction|GetMaximumScore))
    (:then_4
      (CallFunction|JudgementSystem))))

(event EventOnLogout
  (params (ExitingController :type Controller%20Object%20Reference))
  (bind _asplayer_controller (Utilities|Casting|CastToPlayerController ExitingController))
  (Utilities|Array|RemoveItem (Variables|REF|GetPCs) _asplayer_controller))

(event EventOnSwapPlayerControllers
  (params (OldPC :type Player%20Controller%20Object%20Reference) (NewPC :type Player%20Controller%20Object%20Reference))
  (Utilities|Array|Add (Variables|REF|GetPCs) NewPC))

(fn ConstructionScript)

(fn SpawnPlayer
  (params (Controller :type Controller%20Object%20Reference) (CharacterIndex :type Integer) (TeamIndex :type Integer))
  (bind _returnvalue (CallFunction|GetRandomPlayerStart))
  (bind _returnvalue_2 (Pawn|GetControlledPawn Controller))
  (Utilities|IsValid _returnvalue_2
    (:Is%20Valid
      (Actor|DestroyActor _returnvalue_2))
    (:Is%20Not%20Valid
      _))
  (switch int CharacterIndex
    (:0
      (Variables|Default|SetIndex 0)
      (bind _asplayer_controller (Utilities|Casting|CastToPlayerController Controller))
      (Class|PlayerController|ClientSetHUD _asplayer_controller "/Game/Blueprints/UI/BP_PlayerHUD.BP_PlayerHUD_C")
      (bind _returnvalue_3 (Game|SpawnActorfromClass "/Game/Blueprints/Character/Joyce/BP_Joyce.BP_Joyce_C" _returnvalue "AdjustIfPossibleButAlwaysSpawn" 0 1.7e+03 0.0 0))
      (Variables|/Script/KidKing.BaseCharacter|SetTeamIndex _returnvalue_3 TeamIndex)
      (return _returnvalue_3))
    (:1
      (Variables|Default|SetIndex 1)
      (bind _asplayer_controller_2 (Utilities|Casting|CastToPlayerController Controller))
      (Class|PlayerController|ClientSetHUD _asplayer_controller_2 "/Game/Blueprints/UI/BP_PlayerHUD.BP_PlayerHUD_C")
      (bind _returnvalue_4 (Game|SpawnActorfromClass "/Game/Blueprints/Character/Sara/BP_Sara.BP_Sara_C" _returnvalue "AdjustIfPossibleButAlwaysSpawn" 0 1.7e+03 0))
      (Variables|/Script/KidKing.BaseCharacter|SetTeamIndex _returnvalue_4 TeamIndex)
      (return _returnvalue_4))))

(fn GetPlayerStartLocationbyName
  (params (PlayerController :type Controller%20Object%20Reference) (IncomingName :type String))
  (return (Transformation|GetActorTransform (Class|GameModeBase|FindPlayerStart PlayerController IncomingName))))

(fn GetRandomPlayerStart
  (bind _outactors (Actor|GetAllActorsOfClass "/Script/Engine.PlayerStart"))
  (return (Transformation|GetActorTransform (Utilities|Array|Get(acopy) _outactors (Math|Random|RandomIntegerinRange 0 (- (Utilities|Array|Length _outactors) 1))))))