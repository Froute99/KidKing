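; Projectile pickup that grants a power buff through the Gameplay Ability System to the character it hits.
; The construction script drives projectile movement from the Speed and Gravity variables, and BeginPlay makes the sphere ignore the owner while moving.
; On a sphere hit with a BaseCharacter, it applies GE_PowerUp, sends a Buff.Power gameplay event and destroys itself.
; Hits on other actors have no effect.
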(event OnComponentHit(Sphere)
  (params (HitComponent :type Primitive%20Component%20Object%20Reference) (OtherActor :type Actor%20Object%20Reference) (OtherComp :type Primitive%20Component%20Object%20Reference) (NormalImpulse :type Vector :default "0, 0, 0") (Hit :type Hit%20Result%20Structure%20%28by%20ref%29))
  (Variables|Default|SetOther%20Actor OtherActor)
  (CallFunction|BuffBall))

(event Custom|BuffBall
  (bind _asbase_character (Utilities|Casting|CastToBaseCharacter (Variables|Default|GetOther%20Actor)))
  (GameplayEffects|ApplyGameplayEffectToSelf :self (Ability|GetAbilitySystemComponent _asbase_character) :GameplayEffectClass "/Game/Blueprints/Character/Joyce/Ability/Effects/GE_PowerUp.GE_PowerUp_C")
  (Ability|SendGameplayEventtoActor _asbase_character "(TagName=\"Buff.Power\")")
  (Actor|DestroyActor))

(event EventBeginPlay
  (Collision|IgnoreActorwhenMoving (Variables|Default|GetSphere) (Components|GetOwner) true))

(event Collision|EventActorBeginOverlap
  (params (OtherActor :type Actor%20Object%20Reference)))

(event EventTick
  (params (DeltaSeconds :type Float%20%28single-precision%29)))

(fn ConstructionScript
  (bind _projectilemovement (Variables|Default|GetProjectileMovement))
  (Variables|/Script/Engine.ProjectileMovementComponent|SetInitialSpeed _projectilemovement (Variables|ProjectileSetting|GetSpeed))
  (Variables|/Script/Engine.ProjectileMovementComponent|SetMaxSpeed _projectilemovement (Variables|ProjectileSetting|GetSpeed))
  (Variables|/Script/Engine.ProjectileMovementComponent|SetProjectileGravityScale _projectilemovement (Variables|ProjectileSetting|GetGravity)))