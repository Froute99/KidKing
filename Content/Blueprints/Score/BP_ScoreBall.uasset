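; BP_ScoreBall is a projectile ball that awards 100 points to the player whose character it hits.
; The construction script copies Speed and Gravity into ProjectileMovement, and BeginPlay makes the sphere ignore its owner when moving.
; A sphere hit on a BaseCharacter with a BP_KidKingPlayerState adds to PlayerScore, plays a 2D sound and destroys the ball; other hits do nothing.
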(event OnComponentHit(Sphere)
  (params (HitComponent :type Primitive%20Component%20Object%20Reference) (OtherActor :type Actor%20Object%20Reference) (OtherComp :type Primitive%20Component%20Object%20Reference) (NormalImpulse :type Vector :default "0, 0, 0") (Hit :type Hit%20Result%20Structure%20%28by%20ref%29))
  (Variables|Default|SetOther%20Actor OtherActor)
  (CallFunction|ScoreBall))

(event Custom|ScoreBall
  (bind _asbase_character (Utilities|Casting|CastToBaseCharacter (Variables|Default|GetOther%20Actor)))
  (bind _asbp_kid_king_player_state (Utilities|Casting|CastToBP_KidKingPlayerState (Variables|/Script/Engine.Pawn|GetPlayerState _asbase_character)))
  (Variables|/Game/Blueprints/Character/BP_KidKingPlayerState.BP_KidKingPlayerState_C|SetPlayerScore _asbp_kid_king_player_state (+ (Variables|/Game/Blueprints/Character/BP_KidKingPlayerState.BP_KidKingPlayerState_C|GetPlayerScore _asbp_kid_king_player_state) 100))
  (Audio|PlaySound2D "/Game/resource/Sound/Item/effect_notify-84408__online-audio-converter_com_.effect_notify-84408__online-audio-converter_com_" 1.0 1.0 0.0 0 0)
  (Actor|DestroyActor))

(event EventBeginPlay
  (Collision|IgnoreActorwhenMoving (Variables|Default|GetSphere) (Components|GetOwner) true))

(event Collision|EventActorBeginOverlap
  (params (OtherActor :type Actor%20Object%20Reference)))

(event EventTick
  (params (DeltaSeconds :type Float%20%28single-precision%29)))

(fn ConstructionScript
  (bind _projectilemovement (Variables|Default|GetProjectileMovement))
  (Variables|/Script/Engine.ProjectileMovementComponent|SetInitialSpeed _projectilemovement (Variables|ProjectileSetting|GetSpeed))
  (Variables|/Script/Engine.ProjectileMovementComponent|SetMaxSpeed _projectilemovement (Variables|ProjectileSetting|GetSpeed))
  (Variables|/Script/Engine.ProjectileMovementComponent|SetProjectileGravityScale _projectilemovement (Variables|ProjectileSetting|GetGravity)))