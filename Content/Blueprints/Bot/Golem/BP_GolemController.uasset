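; AI controller for the Golem bot that runs its behavior tree and tracks what it sees.
; BeginPlay starts BT_Golem, and perception updates feed HandleSightSense.
; Sight stimuli write the sensed actor to the ChasingTarget blackboard key, or clear it when sight is lost, with debug prints along the way.
; The sensed actor is not filtered, so any perceived actor can become the target.
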(event OnTargetPerceptionUpdated(AIPerception)
  (params (Actor :type Actor%20Object%20Reference) (Stimulus :type AI%20Stimulus%20Structure))
  (CallFunction|HandleSightSense Actor Stimulus))

(event EventBeginPlay
  (AI|RunBehaviorTree "/Game/Blueprints/Bot/Golem/BT_Golem.BT_Golem"))

(fn ConstructionScript)

(fn HandleSightSense
  (params (TargetActor :type Actor%20Object%20Reference%20%28by%20ref%29) (Stimulus :type AI%20Stimulus%20Structure%20%28by%20ref%29))
  (bind _returnvalue (Class|AIPerceptionSystem|GetSenseClassforStimulus Stimulus))
  (if (== _returnvalue "/Script/AIModule.AISense_Sight")
    (if (.bsuccessfullysensed Stimulus)
      (Development|PrintString "Valid")
      (AI|Components|Blackboard|SetValueasObject (Variables|Default|GetBlackboard) (Utilities|Name|MakeLiteralName "ChasingTarget") TargetActor)
      (else
        (Development|PrintString "Not Valid")
        ;[1 1 1] Lose Target from Sight
        (AI|Components|Blackboard|ClearValue (Variables|Default|GetBlackboard) (Utilities|Name|MakeLiteralName "ChasingTarget"))
        (Development|PrintString "Cleared")))
    (else
      (Development|PrintString "Failed to Sense"))))