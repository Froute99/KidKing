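; Golem ability actor for an expanding shock wave that damages characters it reaches.
; On BeginPlay a timeline scales the Sphere component up, then destroys the actor when finished.
; Sphere overlaps loop over BaseCharacter actors with an ability system, applying the shock wave GameplayEffect and sending a Character.Damaged event.
; A single DoOnce gates this, so only the first valid character is hit; an older BP_Joyce-specific branch is unconnected.
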(event OnComponentBeginOverlap(Sphere)
  (params (OverlappedComponent :type Primitive%20Component%20Object%20Reference) (OtherActor :type Actor%20Object%20Reference) (OtherComp :type Primitive%20Component%20Object%20Reference) (OtherBodyIndex :type Integer) (bFromSweep :type Boolean) (SweepResult :type Hit%20Result%20Structure%20%28by%20ref%29))
  (for _array_element (Collision|GetOverlappingActors (Variables|Default|GetSphere) "/Script/KidKing.BaseCharacter" :!class /Script/Engine.PrimitiveComponent)
    (Utilities|IsValid (Ability|GetAbilitySystemComponent _array_element)
      (:Is%20Valid
        (Utilities|FlowControl|DoOnce false
          (:Completed
            (GameplayEffects|ApplyGameplayEffectToTarget :self (Ability|GetAbilitySystemComponent _array_element) :GameplayEffectClass "/Game/Blueprints/Bot/Golem/Ability/BP_GAS_ShockWaveEffect.BP_GAS_ShockWaveEffect_C" :Target (Ability|GetAbilitySystemComponent _array_element))
            (Ability|SendGameplayEventtoActor _array_element "(TagName=\"Character.Damaged\")" (Utilities|Struct|MakeGameplayEventData "(TagName=\"\")" self _array_element 0 0 "()" "(GameplayTags=)" "(GameplayTags=)" 0.0 (Ability|TargetData|AbilityTargetDatafromActor _array_element)))
            (Development|PrintString "ShockWave Valid"))))
      (:Is%20Not%20Valid
        (Development|PrintString "InShockWave")))))

(event EventBeginPlay
  (bind _0_to_1 (Timeline|Timeline Play)
    (:Update
      (Transformation|SetRelativeScale3D (Variables|Default|GetSphere) (Math|Vector|MakeVector (Math|Float|Lerp 1.0 3.5 _0_to_1) (Math|Float|Lerp 1.0 3.5 _0_to_1) (Math|Float|Lerp 1.0 3.5 _0_to_1))))
    (:Finished
      (Actor|DestroyActor))))

(event Collision|EventActorBeginOverlap
  (params (OtherActor :type Actor%20Object%20Reference)))

(event EventTick
  (params (DeltaSeconds :type Float%20%28single-precision%29)))

(fn ConstructionScript)