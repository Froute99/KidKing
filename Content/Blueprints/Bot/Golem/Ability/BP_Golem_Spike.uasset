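; Spike actor for the Golem bot's ability that thrusts out on spawn and damages a character it hits.
; BeginPlay quickly moves the capsule by the spike height along relative X, later destroys it to end the hit window, then destroys the actor.
; On overlap, the first character with an ability system gets a shockwave GameplayEffect and a Character.Damaged event, limited by DoOnce.
; An older BP_Joyce-specific damage branch is left unconnected.
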(event EventBeginPlay
  (bind _capsule (Variables|Default|GetCapsule))
  (Variables|Default|SetInitialLocation (Transformation|GetActorLocation))
  (Components|MoveComponentTo _capsule (Math|Vector|MakeVector (Variables|Default|GetSpikeMaxHeight) 0.0 0.0) "0, 0, 0" false false 0.1 false)
  (Utilities|FlowControl|Delay 1.0)
  (Components|DestroyComponent _capsule)
  (Utilities|FlowControl|Delay 0.6)
  (Actor|DestroyActor))

(event Collision|EventActorBeginOverlap
  (params (OtherActor :type Actor%20Object%20Reference))
  (for _array_element (Collision|GetOverlappingActors (Variables|Default|GetCapsule) "/Script/KidKing.BaseCharacter" :!class /Script/Engine.PrimitiveComponent)
    (Utilities|IsValid (Ability|GetAbilitySystemComponent _array_element)
      (:Is%20Valid
        (Utilities|FlowControl|DoOnce false
          (:Completed
            (GameplayEffects|ApplyGameplayEffectToTarget :self (Ability|GetAbilitySystemComponent _array_element) :GameplayEffectClass "/Game/Blueprints/Bot/Golem/Ability/BP_GAS_ShockWaveEffect.BP_GAS_ShockWaveEffect_C" :Target (Ability|GetAbilitySystemComponent _array_element))
            (Ability|SendGameplayEventtoActor _array_element "(TagName=\"Character.Damaged\")" (Utilities|Struct|MakeGameplayEventData "(TagName=\"\")" self _array_element 0 0 "()" "(GameplayTags=)" "(GameplayTags=)" 0.0 (Ability|TargetData|AbilityTargetDatafromActor _array_element))))))
      (:Is%20Not%20Valid
        (Development|PrintString "Projrctile_AbilityFail")))))

(fn ConstructionScript)