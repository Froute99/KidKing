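; Elder boss bot with a timed spawn-in effect and three attacks: wood spike, leaf storm and default strike.
; Each attack halts movement, plays a montage and spawns a short-lived actor; the spike is telegraphed by a decal.
; Tick registers Character.Damaged gameplay-event waits that set the instigating controller's combat target and update its boss HP widget.
; Tick also polls health, triggering a one-time death that drops score and potion balls.
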(event Custom|OnSkill1
  (bind _scene2 (Variables|Default|GetScene2))
  (bind _returnvalue (Transformation|GetWorldTransform _scene2))
  ;[1 1 1] Skill Wood Spike
  (Variables|/Script/Engine.CharacterMovementComponent|SetMaxWalkSpeed (Variables|Character|GetCharacterMovement) 0.0)
  (Animation|Montage|PlayMontage (Variables|Character|GetMesh) "/Game/Blueprints/Bot/Elder/Animation/ElderSkill01Montage.ElderSkill01Montage"
    (:then
      (bind _returnvalue_2 (Rendering|Decal|SpawnDecalatLocation "/Game/resource/PointDecal/DamageDecal_Mat.DamageDecal_Mat" "5000.000000,5000.000000,5000.000000" (.location (Transformation|GetWorldTransform (Variables|Default|GetScene2))) "-90.000000,0.000000,0.000000" 0.0))
      (Utilities|FlowControl|Delay 7.0)
      (Components|DestroyComponent _returnvalue_2)
      (bind _returnvalue_3 (Game|SpawnActorfromClass "/Game/Blueprints/Bot/Elder/Skill/BP_WoodSpike.BP_WoodSpike_C" (Math|Transform|MakeTransform (.location _returnvalue) "0, 0, 0" "1.000000,1.000000,1.000000") "Undefined" 0 0))
      (Audio|PlaySoundatLocation "/Game/resource/Sound/Attack/WoodSpikeSound.WoodSpikeSound" (.location _returnvalue) "0, 0, 0" 1.0 1.0 0.0 0 0 0 0)
      (Development|PrintString "SpawnSkill01")
      (Utilities|FlowControl|Delay 3.0)
      (Actor|DestroyActor _returnvalue_3))
    (:OnCompleted
      (Variables|/Script/Engine.CharacterMovementComponent|SetMaxWalkSpeed (Variables|Character|GetCharacterMovement) 6e+02))))

(event Custom|OnSkill2
  ;[1 1 1] Skill02 LeafStorm
  (Variables|/Script/Engine.CharacterMovementComponent|SetMaxWalkSpeed (Variables|Character|GetCharacterMovement) 0.0)
  (Animation|Montage|PlayMontage (Variables|Character|GetMesh) "/Game/Blueprints/Bot/Elder/Animation/ElderSkill02Montage.ElderSkill02Montage"
    (:then
      (bind _returnvalue (Actor|GetActorOfClass "/Script/KidKing.BaseCharacter"))
      (bind _returnvalue_2 (Game|SpawnActorfromClass "/Game/Blueprints/Bot/Elder/Skill/BP_LeafStorm.BP_LeafStorm_C" (Transformation|GetWorldTransform (Variables|Default|GetScene)) "Undefined" self 3e+02 0.0 _returnvalue false 0))
      (Development|PrintString "SpawnSkill02")
      (Utilities|FlowControl|Delay 8.0)
      (Actor|DestroyActor _returnvalue_2))
    (:OnCompleted
      (Variables|/Script/Engine.CharacterMovementComponent|SetMaxWalkSpeed (Variables|Character|GetCharacterMovement) 6e+02))))

(event Custom|OnDefaultAttack
  ;[1 1 1] Default Attack
  (Variables|/Script/Engine.CharacterMovementComponent|SetMaxWalkSpeed (Variables|Character|GetCharacterMovement) 0.0)
  (Animation|Montage|PlayMontage (Variables|Character|GetMesh) "/Game/Blueprints/Bot/Elder/Animation/ElderDefaultAttackMontage.ElderDefaultAttackMontage"
    (:then
      (Utilities|FlowControl|Delay 0.5)
      (bind _returnvalue (Game|SpawnActorfromClass "/Game/Blueprints/Bot/Elder/Skill/BP_ElderDefaultAttack.BP_ElderDefaultAttack_C" (Transformation|GetWorldTransform (Variables|Default|GetScene1)) "Undefined" 0 0))
      (Actor|DestroyActor _returnvalue))
    (:OnCompleted
      (Variables|/Script/Engine.CharacterMovementComponent|SetMaxWalkSpeed (Variables|Character|GetCharacterMovement) 6e+02))))

(event Custom|OnSkill1Server
  ;[1 1 1] Skill Wood Spike
  (CallFunction|OnSkill1))

(event Custom|Spawn_NS
  ;[1 1 1] Spawn_NS
  (Variables|/Script/Engine.CharacterMovementComponent|SetMaxWalkSpeed (Variables|Character|GetCharacterMovement) 0.0)
  (Development|SetHiddeninGame (Variables|Character|GetMesh) true false)
  (Audio|PlaySoundatLocation "/Game/resource/Sound/BGM/Spawn.Spawn" (Transformation|GetActorLocation) "0, 0, 0" 1.0 1.0 0.0 0 0 0 0)
  (Niagara|SpawnSystemAttached "/Game/resource/Spawn_NS/Elder/SpawnElder_NS.SpawnElder_NS" (Variables|Default|GetCapsuleComponent) "None" "0.000000,0.000000,-300.000000" "0.000000,-90.000000,0.000000" "KeepRelativeOffset" false)
  (Utilities|FlowControl|Delay 2.2)
  (Development|SetHiddeninGame (Variables|Character|GetMesh) false false)
  (Variables|/Script/Engine.CharacterMovementComponent|SetMaxWalkSpeed (Variables|Character|GetCharacterMovement) 3e+02))

(event Custom|Onskill2Server
  ;[1 1 1] Skill02 LeafStorm
  (CallFunction|OnSkill2))

(event Custom|OnDefaultAttackSever
  ;[1 1 1] Default Attack
  (CallFunction|OnDefaultAttack))

(event Custom|PotionBall
  ;[1 1 1] Score
  (Game|SpawnActorfromClass "/Game/Blueprints/Potion/BP_PotionBall.BP_PotionBall_C" (Math|Transform|MakeTransform (.location (Transformation|GetWorldTransform (Variables|Default|GetScene))) (Math|Rotator|MakeRotator 0.0 0.0 (.yaw (Math|Random|RandomRotator false))) "1.000000,1.000000,1.000000") "Undefined" 0 3e+02 0.5 0))

(event Custom|ScoreBall
  ;[1 1 1] Score
  (if (not (== (Variables|Default|GetScoreIndex) 5)) :!label _label
    (Utilities|FlowControl|Delay 0.2)
    (Game|SpawnActorfromClass "/Game/Blueprints/Score/BP_ScoreBall.BP_ScoreBall_C" (Math|Transform|MakeTransform (.location (Transformation|GetWorldTransform (Variables|Default|GetScene))) (Math|Rotator|MakeRotator 0.0 0.0 (.yaw (Math|Random|RandomRotator false))) "1.000000,1.000000,1.000000") "Undefined" 0 3e+02 0.5 0)
    (Variables|Default|SetScoreIndex (+ (Variables|Default|GetScoreIndex) 1))
    (goto _label)))

(event EventBeginPlay
  (CallFunction|SpawnNS))

(event EventTick
  (params (DeltaSeconds :type Float%20%28single-precision%29))
  (Utilities|FlowControl|Sequence
    (:then_0
      (bind _payload (Ability|Async|WaitGameplayEventToActor 0 "(TagName=\"Character.Damaged\")" true)
        (:then
          (goto _label Reset))
        (:EventReceived
          (Utilities|FlowControl|DoOnce false :!label _label
            (:Completed
              (Utilities|IsValid (.Instigator (Utilities|Struct|BreakGameplayEventData _payload))
                (:Is%20Valid
                  (bind _asbp_test_controller (Utilities|Casting|CastToBP_TestController (Game|GetInstigatorController (.Instigator (Utilities|Struct|BreakGameplayEventData _payload))))
                    (:then
                      (Variables|/Game/Blueprints/Character/BP_TestController.BP_TestController_C|SetCombatTarget _asbp_test_controller self)
                      (Default|OnDamaged (Variables|/Game/Blueprints/UI/BP_PlayerHUD.BP_PlayerHUD_C|GetBossHpWidget (Variables|/Game/Blueprints/Character/BP_TestController.BP_TestController_C|GetREF%20PlayerHUD _asbp_test_controller))))
                    (:CastFailed
                      (Development|PrintString "Not Valid / Cast Failed" :!label _label_2))))
                (:Is%20Not%20Valid
                  (goto _label_2))))))))
    (:then_1
      (if (<= (Class|BotCharacterBase|GetHealth) 0.0)
        (Utilities|FlowControl|DoOnce false
          (:Completed
            (CallFunction|Death)))))))

(fn ConstructionScript)

(fn Death
  (Variables|/Script/Engine.CharacterMovementComponent|SetMaxWalkSpeed (Variables|Character|GetCharacterMovement) 0.0)
  (Animation|PlayAnimMontage "/Game/Blueprints/Bot/Elder/Animation/ElderDieMontage.ElderDieMontage" 1.0 "None")
  (CallFunction|ScoreBall)
  (CallFunction|PotionBall)
  (Actor|SetLifeSpan 1.5))

(fn GetActorObject
  (return (AI|Components|Blackboard|GetValueasObject (AI|GetBlackboard (AI|GetAIController self)) (Utilities|Name|MakeLiteralName "ChasingTarget"))))