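; BP_MiniGolem is a mini golem bot Blueprint that implements a melee attack through its OnAttack event.
; OnAttack starts the attack montage, then immediately runs SphereCollision, a debug-drawn pawn sphere trace forward by AttackRange.
; The hit actor's own ability system applies GE_MiniGolemAttack to itself, and the actor receives a Character.Damaged gameplay event, with no hit check.
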(event Custom|OnAttack
  (Utilities|FlowControl|Sequence
    (:then_0
      (Animation|Montage|PlayMontage (Variables|Character|GetMesh) "/Game/Blueprints/Bot/MiniGolem/Animation/MiniGolemDefaultAttck.MiniGolemDefaultAttck"))
    (:then_1
      (bind _outhit (CallFunction|SphereCollision))
      (GameplayEffects|ApplyGameplayEffectToTarget :self (Ability|GetAbilitySystemComponent (.HitActor (Collision|BreakHitResult _outhit))) :GameplayEffectClass "/Game/Blueprints/Bot/MiniGolem/Ability/GE_MiniGolemAttack.GE_MiniGolemAttack_C" :Target (Ability|GetAbilitySystemComponent (.HitActor (Collision|BreakHitResult _outhit))))
      (Ability|SendGameplayEventtoActor (.HitActor (Collision|BreakHitResult _outhit)) "(TagName=\"Character.Damaged\")"))))

(event EventBeginPlay)

(event Collision|EventActorBeginOverlap
  (params (OtherActor :type Actor%20Object%20Reference)))

(event EventTick
  (params (DeltaSeconds :type Float%20%28single-precision%29)))

(fn ConstructionScript)

(fn SphereCollision
  (bind _returnvalue (Transformation|GetActorLocation))
  (bind _outhit (Collision|SphereTraceForObjects _returnvalue (+ _returnvalue (* (Math|Vector|GetForwardVector (Transformation|GetActorRotation)) (Variables|Default|GetAttackRange))) 5e+01 (Utilities|Array|MakeArray "ObjectTypeQuery3") false 0 "ForDuration" true "(R=1.000000,G=0.000000,B=0.000000,A=1.000000)" "(R=0.000000,G=1.000000,B=0.000000,A=1.000000)" 1.0))
  (return _outhit))