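; MiniElder enemy bot that melee-attacks through the Gameplay Ability System and drops score and potion balls on death.
; OnAttack sets the IsAttacking blackboard key during its montage, while a forward sphere trace applies GE_MiniGolemAttack and sends Character.Damaged.
; Tick updates the health bar, triggers Die at zero health and creates a damage-event wait each frame.
; Damage handling only prints debug text; hit reaction nodes are disconnected.
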(event Custom|OnAttack
  ;[1 1 1] Attack
  (CallFunction|LookAttacking)
  (Utilities|FlowControl|Sequence
    (:then_0
      (Animation|Montage|PlayMontage (Variables|Character|GetMesh) "/Game/Blueprints/Bot/MiniElder/Animation/MiniElderAttack_Montage.MiniElderAttack_Montage"
        (:OnCompleted
          (CallFunction|ReleaseAttacking))))
    (:then_1
      (bind _outhit (CallFunction|SphereCollision))
      (GameplayEffects|ApplyGameplayEffectToTarget :self (Ability|GetAbilitySystemComponent (.HitActor (Collision|BreakHitResult _outhit))) :GameplayEffectClass "/Game/Blueprints/Bot/MiniGolem/Ability/GE_MiniGolemAttack.GE_MiniGolemAttack_C" :Target (Ability|GetAbilitySystemComponent (.HitActor (Collision|BreakHitResult _outhit))))
      (Ability|SendGameplayEventtoActor (.HitActor (Collision|BreakHitResult _outhit)) "(TagName=\"Character.Damaged\")"))))

(event Custom|ScoreBall
  ;[1 1 1] Drop
  (Utilities|FlowControl|Delay 0.5)
  (Game|SpawnActorfromClass "/Game/Blueprints/Score/BP_ScoreBall.BP_ScoreBall_C" (Math|Transform|MakeTransform (.location (Transformation|GetWorldTransform (Variables|Default|GetScene))) (Math|Rotator|MakeRotator 0.0 0.0 (.yaw (Math|Random|RandomRotator false))) "1.000000,1.000000,1.000000") "Undefined" 0 3e+02 0.5 0))

(event Custom|PotionBall
  ;[1 1 1] Drop
  (Utilities|FlowControl|Delay 0.5)
  (Game|SpawnActorfromClass "/Game/Blueprints/Potion/BP_PotionBall.BP_PotionBall_C" (Math|Transform|MakeTransform (.location (Transformation|GetWorldTransform (Variables|Default|GetScene))) (Math|Rotator|MakeRotator 0.0 0.0 (.yaw (Math|Random|RandomRotator false))) "1.000000,1.000000,1.000000") "Undefined" 0 3e+02 0.5 0))

(event EventBeginPlay)

(event Collision|EventActorBeginOverlap
  (params (OtherActor :type Actor%20Object%20Reference)))

(event EventTick
  (params (DeltaSeconds :type Float%20%28single-precision%29))
  (Utilities|FlowControl|Sequence
    (:then_0
      (bind _payload (Ability|Async|WaitGameplayEventToActor 0 "(TagName=\"Character.Damaged\")" true)
        (:then
          (goto _label Reset))
        (:EventReceived
          (Utilities|FlowControl|DoOnce false :!label _label
            (:Completed
              (Development|PrintString (Utilities|String|ToString(Float) (Class|BotCharacterBase|GetHealth)))
              (Utilities|IsValid (.Instigator (Utilities|Struct|BreakGameplayEventData _payload))
                (:Is%20Valid
                  (bind _asbp_test_controller (Utilities|Casting|CastToBP_TestController (Game|GetInstigatorController (.Instigator (Utilities|Struct|BreakGameplayEventData _payload))))
                    (:CastFailed
                      _)))
                (:Is%20Not%20Valid
                  _))
              (Development|PrintString "Not Valid / Cast Failed"))))))
    (:then_1
      (if (<= (Class|BotCharacterBase|GetHealth) 0.0)
        (Utilities|FlowControl|DoOnce false
          (:Completed
            (CallFunction|Die)))))
    (:then_2
      (bind _asbot_healthbar (Utilities|Casting|CastToBot_Healthbar (UserInterface|GetWidget (Variables|Default|GetHealth%20bar))))
      (Progress|SetPercent (Variables|/Game/Blueprints/UI/Bot_Healthbar.Bot_Healthbar_C|GetHealthBar _asbot_healthbar) (/ (Class|BotCharacterBase|GetHealth) (Class|BotCharacterBase|GetMaxHealth))))))

(fn ConstructionScript)

(fn LookAttacking
  (AI|Components|Blackboard|SetValueasBool (AI|GetBlackboard (AI|GetAIController self)) (Utilities|Name|MakeLiteralName "IsAttacking") true))

(fn ReleaseAttacking
  (AI|Components|Blackboard|SetValueasBool (AI|GetBlackboard (AI|GetAIController self)) (Utilities|Name|MakeLiteralName "IsAttacking") false))

(fn SphereCollision
  (bind _returnvalue (Transformation|GetActorLocation))
  (bind _outhit (Collision|SphereTraceForObjects _returnvalue (+ _returnvalue (* (Math|Vector|GetForwardVector (Transformation|GetActorRotation)) (Variables|Default|GetAttackRange))) 1e+02 (Utilities|Array|MakeArray "ObjectTypeQuery3") false 0 "ForDuration" true "(R=1.000000,G=0.000000,B=0.000000,A=1.000000)" "(R=0.000000,G=1.000000,B=0.000000,A=1.000000)" 1.0))
  (return _outhit))

(fn Die
  (Variables|/Script/Engine.CharacterMovementComponent|SetMaxWalkSpeed (Variables|Character|GetCharacterMovement) 0.0)
  (Animation|PlayAnimMontage "/Game/Blueprints/Bot/MiniElder/Animation/MiniElderDie.MiniElderDie" 1.0 "None")
  (CallFunction|ScoreBall)
  (CallFunction|PotionBall)
  (Actor|SetLifeSpan 1.5))