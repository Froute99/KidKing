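; Golem bot character with a default attack and three skills: shockwave, meteor and stone spike.
; Each attack plays a montage between lock and release calls, with delays timing the spawned skill actors.
; The default attack applies a GAS damage effect and sends a Character.Damaged event to the hit actor.
; Tick prints health and registers a damage-event wait; locking, collision and targeting functions are empty stubs here.
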(event Custom|OnAttack
  (Utilities|FlowControl|Sequence
    (:then_0
      (CallFunction|LockAttacking)
      (bind _returnvalue (Animation|PlayAnimMontage "/Game/BluePrint/Bot/Golem/Golem_DefaultAttack.Golem_DefaultAttack" 1.0 "None"))
      (Utilities|FlowControl|Delay _returnvalue)
      (CallFunction|ReleaseAttacking)
      (Development|PrintString "Golem Default Attack Completed"))
    (:then_1
      (bind _outhit (CallFunction|SphereCollision))
      (GameplayEffects|ApplyGameplayEffectToTarget :self (Ability|GetAbilitySystemComponent (.HitActor (Collision|BreakHitResult _outhit))) :GameplayEffectClass "/Game/BluePrint/Character/Joyce/Ability/BP_GAS_DamageEffect.BP_GAS_DamageEffect_C" :Target (Ability|GetAbilitySystemComponent (.HitActor (Collision|BreakHitResult _outhit))))
      (Ability|SendGameplayEventtoActor (.HitActor (Collision|BreakHitResult _outhit)) "(TagName=\"Character.Damaged\")" (Utilities|Struct|MakeGameplayEventData "(TagName=\"\")" self (.HitActor (Collision|BreakHitResult _outhit)) 0 0 "()" "(GameplayTags=)" "(GameplayTags=)" 0.0 (Ability|TargetData|AbilityTargetDatafromActor (.HitActor (Collision|BreakHitResult _outhit))))))))

(event Custom|OnSkill1
  ;[1 1 1] Skill1 / Shockwave
  (Utilities|FlowControl|Sequence
    (:then_0
      (CallFunction|LockAttacking)
      (bind _returnvalue (Animation|PlayAnimMontage "/Game/BluePrint/Bot/Golem/Golem_ShockWave.Golem_ShockWave" 1.0 "None"))
      (Utilities|FlowControl|Delay _returnvalue)
      (CallFunction|ReleaseAttacking)
      (Development|PrintString "Golem Skill1 Completed"))
    (:then_1
      (Utilities|FlowControl|Delay 2.1)
      (Game|SpawnActorfromClass "/Game/BluePrint/Bot/Golem/Ability/BP_ShockWave.BP_ShockWave_C" (Math|Transform|MakeTransform (Transformation|GetActorLocation) "0, 0, 0" "1.000000,1.000000,1.000000") "Undefined" 0 0))))

(event Custom|OnSkill2
  (bind _self self)
  ;[1 1 1] Skill2 / Meteor
  (Utilities|FlowControl|Sequence
    (:then_0
      (CallFunction|LockAttacking)
      (bind _returnvalue (Animation|PlayAnimMontage "/Game/BluePrint/Bot/Golem/Golem_Meteor.Golem_Meteor" 1.0 "None"))
      (Utilities|FlowControl|Delay _returnvalue)
      (CallFunction|ReleaseAttacking)
      (Development|PrintString "Golem Skill2 Completed"))
    (:then_1
      (bind _returnvalue_2 (Game|SpawnActorfromClass "/Game/BluePrint/Bot/Golem/Ability/BP_Meteor.BP_Meteor_C" (Math|Transform|MakeTransform (+ (Transformation|GetActorLocation) (Math|Vector|MakeVector (* (Math|Random|RandomFloat) 1.2e+03) (* 1.2e+03 (Math|Random|RandomFloat)) 1e+04)) "0, 0, 0" "5.000000,5.000000,5.000000") "AdjustIfPossibleButAlwaysSpawn" _self _self))
      (bind _returnvalue_3 (CallFunction|GetTargetLocation))
      (Utilities|FlowControl|Delay 1.65)
      (Components|MoveComponentTo (Variables|/Game/BluePrint/Bot/Golem/Ability/BP_Meteor.BP_Meteor_C|GetSphere _returnvalue_2) (Math|Vector|MakeVector (.X (Class|KismetMathLibrary|BreakVector3f _returnvalue_3)) (.Y (Class|KismetMathLibrary|BreakVector3f _returnvalue_3)) (- (.Z (Class|KismetMathLibrary|BreakVector3f _returnvalue_3)) 8e+01)) "0, 0, 0" false false 1.0 false)
      (Default|Blast _returnvalue_2 (Math|Vector|MakeVector (.X (Class|KismetMathLibrary|BreakVector3f _returnvalue_3)) (.Y (Class|KismetMathLibrary|BreakVector3f _returnvalue_3)) (- (.Z (Class|KismetMathLibrary|BreakVector3f _returnvalue_3)) 8e+01)))
      (Utilities|FlowControl|Delay 5.0)
      (Actor|DestroyActor _returnvalue_2))))

(event Custom|OnSkill3
  (bind _returnvalue (Transformation|GetActorLocation))
  (bind _returnvalue_2 (Transformation|GetActorForwardVector))
  (bind _returnvalue_3 (CallFunction|GetActorObject))
  (bind _ascharacter (Utilities|Casting|CastToCharacter _returnvalue_3))
  (bind _returnvalue_4 (* _returnvalue_2 2.5e+02))
  (bind _returnvalue_5 (+ _returnvalue _returnvalue_4))
  (bind _capsulecomponent (Variables|/Script/Engine.Character|GetCapsuleComponent _ascharacter))
  (bind (_origin _boxextent _sphereradius) (Collision|GetComponentBounds _capsulecomponent))
  ;[1 1 1] Skill3 / Stone Spike
  (CallFunction|LockAttacking)
  (bind _returnvalue_6 (Animation|PlayAnimMontage "/Game/BluePrint/Bot/Golem/Golem_Spike.Golem_Spike" 1.0 "None"))
  (bind _output_get (Variables|Default|SetSpikeTargetLocation (Math|Vector|MakeVector (.x _returnvalue_5) (.y _returnvalue_5) (- (.Z (Class|KismetMathLibrary|BreakVector3f _origin)) _sphereradius))))
  (Utilities|FlowControl|Delay 0.75)
  (Game|SpawnActorfromClass "/Game/BluePrint/Bot/Golem/Ability/BP_Golem_Spike.BP_Golem_Spike_C" (Math|Transform|MakeTransform _output_get "0, 0, 0" "1.000000,1.000000,1.000000") "Undefined" 0 0)
  (Utilities|FlowControl|Delay _returnvalue_6)
  (CallFunction|ReleaseAttacking))

(event EventBeginPlay)

(event Collision|EventActorBeginOverlap
  (params (OtherActor :type Actor%20Object%20Reference)))

(event EventTick
  (params (DeltaSeconds :type Float%20%28single-precision%29))
  (Utilities|FlowControl|Sequence
    (:then_0
      (Ability|Async|WaitGameplayEventToActor 0 "(TagName=\"Character.Damaged\")" true
        (:EventReceived
          (Development|PrintString "Golem Damaged"))))
    (:then_1
      (Development|PrintString (Utilities|String|ToString(Float) (Class|BotCharacterBase|GetHealth))))))

(fn ConstructionScript)

(fn LockAttacking)

(fn ReleaseAttacking)

(fn SphereCollision
  (return ""))

(fn GetTargetLocation
  (return "0, 0, 0"))

(fn GetActorObject
  (return 0))