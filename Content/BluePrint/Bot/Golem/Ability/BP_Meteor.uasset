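; BP_Meteor is a Golem ability actor for a meteor strike aimed at a Character.
; Trace line-traces toward just below the Character and places a damage-area decal at the impact.
; Blast plays sound, spawns Fire and applies GAS damage, a Damaged event and tag-activated knockback to BP_Joyce actors overlapping the Sphere.
; The sequence chaining Trace, sphere movement, Blast and self-destruction is disconnected, and BeginPlay is empty.
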(event Custom|Trace
  (bind _character (Variables|Default|GetCharacter))
  (bind _returnvalue (Transformation|GetActorLocation _character))
  (bind _outhit (Collision|LineTraceByChannel (Transformation|GetActorLocation) (Math|Vector|MakeVector (.x _returnvalue) (.y _returnvalue) (- (.z _returnvalue) 1e+02)) "TraceTypeQuery1" false 0 "None"))
  (bind _output_get (Variables|Default|SetImpact%20Point (.ImpactPoint (Collision|BreakHitResult _outhit))))
  (bind _returnvalue_2 (Rendering|Decal|SpawnDecalatLocation "/Game/resource/Meteoroid/DemageArea_Inst.DemageArea_Inst" "300.000000,300.000000,300.000000" _output_get (Math|Conversions|RotationFromXVector (.ImpactNormal (Collision|BreakHitResult _outhit))) 0.0))
  (Variables|Default|SetDemageDecal _returnvalue_2))

(event Custom|Blast
  (params (TargetLocation :type Vector))
  (Audio|PlaySoundatLocation 0 TargetLocation "0, 0, 0" 1.0 1.0 0.0 0 0 0 0)
  (bind _returnvalue (Game|SpawnActorfromClass "/Game/resource/Meteoroid/Fire.Fire_C" (Math|Transform|MakeTransform TargetLocation "0, 0, 0" "1.000000,1.000000,1.000000") "Undefined" 0 0))
  (for _array_element (Collision|GetOverlappingActors (Variables|Default|GetSphere) "/Game/BluePrint/Character/Joyce/BP_Joyce.BP_Joyce_C" :!class /Script/Engine.PrimitiveComponent)
    (GameplayEffects|ApplyGameplayEffectToTarget :self (Ability|GetAbilitySystemComponent _array_element) :GameplayEffectClass "/Game/BluePrint/Bot/Golem/Ability/BP_GAS_MeteorDamageEffect.BP_GAS_MeteorDamageEffect_C" :Target (Ability|GetAbilitySystemComponent _array_element))
    (Ability|SendGameplayEventtoActor _array_element "(TagName=\"Character.Damaged\")" (Utilities|Struct|MakeGameplayEventData "(TagName=\"\")" self 0 0 0 "()" "(GameplayTags=)" "(GameplayTags=)" 0.0 (Ability|TargetData|AbilityTargetDatafromActor 0)))
    (Abilities|TryActivateAbilitiesbyTag (Ability|GetAbilitySystemComponent _array_element) (Variables|Default|GetKnockback%20Tag) true)
    (Utilities|FlowControl|Delay 3.0)
    (Actor|DestroyActor _returnvalue)))

(event EventBeginPlay)

(event Collision|EventActorBeginOverlap
  (params (OtherActor :type Actor%20Object%20Reference)))

(event EventTick
  (params (DeltaSeconds :type Float%20%28single-precision%29)))

(fn ConstructionScript)