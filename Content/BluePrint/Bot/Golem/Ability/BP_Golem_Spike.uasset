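; BP_Golem_Spike is a short-lived Golem ability hazard that damages BP_Joyce on overlap.
; On BeginPlay it quickly slides its capsule along relative X to SpikeMaxHeight, removes the capsule after a delay, then destroys itself shortly after.
; An overlap applies the GAS shockwave effect through Joyce's own ability system component and sends a Character.Damaged gameplay event with the spike as instigator.
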(event EventBeginPlay
  (bind _capsule (Variables|Default|GetCapsule))
  (Variables|Default|SetInitialLocation (Transformation|GetActorLocation))
  (Components|MoveComponentTo _capsule (Math|Vector|MakeVector (Variables|Default|GetSpikeMaxHeight) 0.0 0.0) "0, 0, 0" false false 0.1 false)
  (Utilities|FlowControl|Delay 1.0)
  (Components|DestroyComponent _capsule)
  (Utilities|FlowControl|Delay 0.6)
  (Actor|DestroyActor))

(event Collision|EventActorBeginOverlap
  (params (OtherActor :type Actor%20Object%20Reference))
  (bind (_asbp_joyce _bsuccess) (Utilities|Casting|CastToBP_Joyce OtherActor))
  (bind _returnvalue (Ability|GetAbilitySystemComponent _asbp_joyce))
  (if _bsuccess
    (GameplayEffects|ApplyGameplayEffectToTarget :self _returnvalue :GameplayEffectClass "/Game/BluePrint/Bot/Golem/Ability/BP_GAS_ShockWaveEffect.BP_GAS_ShockWaveEffect_C" :Target _returnvalue)
    (Ability|SendGameplayEventtoActor _asbp_joyce "(TagName=\"Character.Damaged\")" (Utilities|Struct|MakeGameplayEventData "(TagName=\"\")" self _asbp_joyce 0 0 "()" "(GameplayTags=)" "(GameplayTags=)" 0.0 (Ability|TargetData|AbilityTargetDatafromActor _asbp_joyce)))))

(fn ConstructionScript)