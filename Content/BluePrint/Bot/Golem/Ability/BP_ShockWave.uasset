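; Shockwave hazard actor, filed under the Golem's abilities, that hits BP_Joyce as it expands.
; On BeginPlay a timeline scales its Sphere up to 3.5x, then the actor destroys itself.
; Sphere overlaps with Joyce apply BP_GAS_ShockWaveEffect through her own ability system component as both source and target.
; They also send her a Character.Damaged gameplay event with the shockwave as instigator, plus a debug print.
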(event OnComponentBeginOverlap(Sphere)
  (params (OverlappedComponent :type Primitive%20Component%20Object%20Reference) (OtherActor :type Actor%20Object%20Reference) (OtherComp :type Primitive%20Component%20Object%20Reference) (OtherBodyIndex :type Integer) (bFromSweep :type Boolean) (SweepResult :type Hit%20Result%20Structure%20%28by%20ref%29))
  (bind _asbp_joyce (Utilities|Casting|CastToBP_Joyce OtherActor))
  (Utilities|IsValid _asbp_joyce
    (:Is%20Valid
      (GameplayEffects|ApplyGameplayEffectToTarget :self (Ability|GetAbilitySystemComponent _asbp_joyce) :GameplayEffectClass "/Game/BluePrint/Bot/Golem/Ability/BP_GAS_ShockWaveEffect.BP_GAS_ShockWaveEffect_C" :Target (Ability|GetAbilitySystemComponent _asbp_joyce))
      (Ability|SendGameplayEventtoActor _asbp_joyce "(TagName=\"Character.Damaged\")" (Utilities|Struct|MakeGameplayEventData "(TagName=\"\")" self _asbp_joyce 0 0 "()" "(GameplayTags=)" "(GameplayTags=)" 0.0 (Ability|TargetData|AbilityTargetDatafromActor _asbp_joyce)))
      (Development|PrintString "ShockWave Valid"))))

(event EventBeginPlay
  (bind _0_to_1 (Timeline|Timeline Play)
    (:Update
      (Transformation|SetRelativeScale3D (Variables|Default|GetSphere) (Math|Vector|MakeVector (Math|Float|Lerp 1.0 3.5 _0_to_1) (Math|Float|Lerp 1.0 3.5 _0_to_1) (Math|Float|Lerp 1.0 3.5 _0_to_1))))
    (:Finished
      (Actor|DestroyActor))))

(event Collision|EventActorBeginOverlap
  (params (OtherActor :type Actor%20Object%20Reference)))

(event EventTick
  (params (DeltaSeconds :type Float%20%28single-precision%29)))

(fn ConstructionScript)