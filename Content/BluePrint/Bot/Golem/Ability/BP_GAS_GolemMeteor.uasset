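; Gameplay ability that runs the Golem bot's meteor attack.
; On activation it waits for instant target data from a meteor target actor, starting just ahead of the Golem.
; Valid data commits the ability, then the authority builds a set-by-caller damage effect spec, though the graph never applies it or ends the ability there.
; Non-authority instances end the ability, while cancelled targeting or a failed commit cancels it.
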(event Ability|EventActivateAbility
  (bind _returnvalue (Class|GameplayAbility|MakeTargetLocationInfofromOwnerActor))
  (Variables|Default|SetOwner (.AsBP%20Golem (Utilities|Casting|CastToBP_Golem (Ability|GetAvatarActorfromActorInfo))))
  (|WaitTargetData :ConfirmationType "Instant" :Class "/Game/BluePrint/Bot/Golem/Ability/BP_GAS_MeteorTarget.BP_GAS_MeteorTarget_C" :MaxRange 5e+02 :StartLocation (Utilities|Struct|MakeGameplayAbilityTargetingLocationInfo (.locationtype _returnvalue) (Math|Transform|MakeTransform (+ (Transformation|GetActorForwardVector (Variables|Default|GetOwner)) (.location (.literaltransform _returnvalue))) (.rotation (.literaltransform _returnvalue)) (.scale (.literaltransform _returnvalue))) (.sourceactor _returnvalue) (.sourcecomponent _returnvalue) (.sourceability _returnvalue) (.sourcesocketname _returnvalue)) :ReticleClass 0
    (:ValidData
      (bind _returnvalue_2 (Ability|CommitAbility))
      (if _returnvalue_2
        (if (Ability|HasAuthority (Variables|Default|GetOwner))
          ;[1 1 1] Apply Damage Effect
          (Ability|GameplayEffect|AssignTagSetbyCallerMagnitude (Ability|MakeOutgoingGameplayEffectSpec (Variables|Default|GetDamage%20Gameplay%20Effect)) "(TagName=\"Data.Meteor.Damage\")" 3e+01)
          (else
            (Ability|EndAbility)))
        (else
          (Ability|CancelAbility :!label _label))))
    (:Cancelled
      (goto _label))))

(event Ability|EventOnEndAbility
  (params (bWasCancelled :type Boolean)))