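; Golem enemy character Blueprint that provides attack events and a range check, with no callers in this graph.
; Default, shockwave and meteor attack events each play their own montage.
; CanAttackPlayer sets CanAttack from a debug-drawn forward sphere trace for any Pawn.
; A separate Meteor event spawns a scaled-up Meteor after a delay if the player is grounded, taking only height from player location; X/Y are player forward-vector components plus fixed offsets.
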(event Custom|Meteor
  (bind _returnvalue (Game|GetPlayerCharacter 0))
  (bind _asnice_clean_character (Utilities|Casting|CastToNiceCleanCharacter _returnvalue))
  (bind _returnvalue_2 (Transformation|GetActorRotation _asnice_clean_character))
  (bind _returnvalue_3 (Math|Vector|GetForwardVector _returnvalue_2))
  (if (AI|Components|NavMovement|IsMovingonGround (Variables|/Script/Engine.Character|GetCharacterMovement _asnice_clean_character))
    (Utilities|FlowControl|Delay 3.0)
    (Game|SpawnActorfromClass "/Game/resource/Meteoroid/Meteor.Meteor_C" (Math|Transform|MakeTransform (Math|Vector|MakeVector (+ (.x _returnvalue_3) 1e+04) (+ (.y _returnvalue_3) 5e+03) (+ (.z (Transformation|GetActorLocation _asnice_clean_character)) 5e+03)) "0, 0, 0" "5.000000,5.000000,5.000000") "Undefined" 0 0)))

(event Custom|CanAttackPlayer
  (bind _returnvalue (Transformation|GetActorLocation))
  (bind _returnvalue_2 (Collision|SphereTraceForObjects _returnvalue (+ _returnvalue (* (Math|Vector|GetForwardVector (Transformation|GetActorRotation)) 2.5e+02)) 3.5e+02 (Utilities|Array|MakeArray "ObjectTypeQuery3") false 0 "ForDuration"))
  (if _returnvalue_2
    (Variables|Default|SetCanAttack true)
    (else
      (Variables|Default|SetCanAttack false))))

(event Custom|ShokeWaveAttack
  (Animation|PlayAnimMontage "/Game/BluePrint/Bot/Golem/Golem_ShokeWave.Golem_ShokeWave" 1.0 "None"))

(event Custom|MeteorAttack
  (Animation|PlayAnimMontage "/Game/BluePrint/Bot/Golem/Golem_Meteor.Golem_Meteor" 1.0 "None"))

(event Custom|DefaultAttack
  (Animation|PlayAnimMontage "/Game/BluePrint/Bot/Golem/Golem_DefaultAttack.Golem_DefaultAttack" 1.0 "None"))

(event EventBeginPlay)

(event Collision|EventActorBeginOverlap
  (params (OtherActor :type Actor%20Object%20Reference)))

(event EventTick
  (params (DeltaSeconds :type Float%20%28single-precision%29)))

(fn ConstructionScript)