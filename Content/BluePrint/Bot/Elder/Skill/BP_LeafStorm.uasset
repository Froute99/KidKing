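; Leaf Storm projectile for the Elder bot's skill, which chases a target and damages characters it overlaps.
; The construction script sets speed, gravity and optional homing, while Tick re-aims velocity at any valid Target using X/Y positions, regardless of the homing flag.
; Box overlap plays a sound and applies a GAS damage effect to every overlapping BaseCharacter with an ability system, without destroying the projectile.
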(event OnComponentBeginOverlap(BoxCollision)
  (params (OverlappedComponent :type Primitive%20Component%20Object%20Reference) (OtherActor :type Actor%20Object%20Reference) (OtherComp :type Primitive%20Component%20Object%20Reference) (OtherBodyIndex :type Integer) (bFromSweep :type Boolean) (SweepResult :type Hit%20Result%20Structure%20%28by%20ref%29))
  (Audio|PlaySoundatLocation 0 "0, 0, 0" "0, 0, 0" 1.0 1.0 0.0 0 0 0 0)
  (for _array_element (Collision|GetOverlappingActors (Variables|Default|GetBoxCollision) "/Script/KidKing.BaseCharacter" :!class /Script/Engine.PrimitiveComponent)
    (Utilities|IsValid (Ability|GetAbilitySystemComponent _array_element)
      (:Is%20Valid
        (GameplayEffects|ApplyGameplayEffectToTarget :self (Ability|GetAbilitySystemComponent _array_element) :GameplayEffectClass "/Game/BluePrint/Bot/Elder/Ability/BP_GAS_LeafStormDamageEffect.BP_GAS_LeafStormDamageEffect_C" :Target (Ability|GetAbilitySystemComponent _array_element)))
      (:Is%20Not%20Valid
        (Development|PrintString "Projrctile_AbilityFail")))))

(event Custom|RotateToTarget
  (bind _returnvalue (Transformation|GetActorLocation))
  (bind _target (Variables|ProjectileSetting|GetTarget))
  (bind _returnvalue_2 (Transformation|GetActorLocation _target))
  (Variables|/Script/Engine.MovementComponent|SetVelocity (Variables|Default|GetProjectileMovement) (* (Math|Vector|GetUnitDirection(Vector) (Math|Vector|MakeVector (.x _returnvalue) (.y _returnvalue) 0.0) (Math|Vector|MakeVector (.x _returnvalue_2) (.y _returnvalue_2) 0.0)) (Variables|ProjectileSetting|GetSpeed))))

(event EventBeginPlay
  (Collision|IgnoreActorwhenMoving (Variables|Default|GetBoxCollision) (Components|GetOwner) true))

(event Collision|EventActorBeginOverlap
  (params (OtherActor :type Actor%20Object%20Reference)))

(event EventTick
  (params (DeltaSeconds :type Float%20%28single-precision%29))
  (Variables|ProjectileSetting|GetTarget
    (:then
      (CallFunction|RotatetoTarget))
    (:else)))

(fn ConstructionScript
  (bind _projectilemovement (Variables|Default|GetProjectileMovement))
  (Variables|/Script/Engine.ProjectileMovementComponent|SetInitialSpeed _projectilemovement (Variables|ProjectileSetting|GetSpeed))
  (Variables|/Script/Engine.ProjectileMovementComponent|SetMaxSpeed _projectilemovement (Variables|ProjectileSetting|GetSpeed))
  (Variables|/Script/Engine.ProjectileMovementComponent|SetProjectileGravityScale _projectilemovement (Variables|ProjectileSetting|GetGravity))
  (Variables|ProjectileSetting|GetTarget
    (:then
      (if (Variables|ProjectileSetting|GetIsHoming)
        (Variables|/Script/Engine.ProjectileMovementComponent|SetbIsHomingProjectile _projectilemovement true)
        (Variables|/Script/Engine.ProjectileMovementComponent|SetHomingTargetComponent _projectilemovement (Variables|/Script/Engine.Actor|GetRootComponent (Variables|ProjectileSetting|GetTarget)))))
    (:else)))