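; CharacterSelector is the character selection actor that previews four Joyce skins (default, pink, green, mint) and records the chosen one.
; On BeginPlay it creates the selection widget, hands it a self-reference and adds it to the viewport.
; Each skin event stores its index and toggles component visibility, using the inverse of the Selected flag for its own variant.
; It then sends the skin index and BlueOrRed value to the GameInstance for saving.
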(event Custom|Udate%20Character%20Data
  (Class|InstanceInterface|SaveCharacterData(Message) (Game|GetGameInstance) (Variables|Default|GetBlue%20Or%20Red) (Variables|Default|GetSelected%20Skin)))

(event Custom|Selected%20Pink
  (params (Selected :type Boolean))
  (Variables|Default|SetSelected%20Skin 1)
  (Rendering|SetVisibility (Variables|Default|GetJoyce) Selected false)
  (Rendering|SetVisibility (Variables|Default|GetJoyce_Pink) (not Selected) false)
  (Rendering|SetVisibility (Variables|Default|GetJoyce_Green) Selected false)
  (Rendering|SetVisibility (Variables|Default|GetJoyce_Mint) Selected false)
  (CallFunction|UdateCharacterData))

(event Custom|joyce%20selected
  (params (selected :type Boolean))
  (Variables|Default|SetSelected%20Skin 0)
  (Rendering|SetVisibility (Variables|Default|GetJoyce) (not selected) false)
  (Rendering|SetVisibility (Variables|Default|GetJoyce_Pink) selected false)
  (Rendering|SetVisibility (Variables|Default|GetJoyce_Green) selected false)
  (Rendering|SetVisibility (Variables|Default|GetJoyce_Mint) selected false)
  (CallFunction|UdateCharacterData))

(event Custom|Selected%20Green
  (params (Selected :type Boolean))
  (Variables|Default|SetSelected%20Skin 3)
  (Rendering|SetVisibility (Variables|Default|GetJoyce) Selected false)
  (Rendering|SetVisibility (Variables|Default|GetJoyce_Pink) Selected false)
  (Rendering|SetVisibility (Variables|Default|GetJoyce_Green) (not Selected) false)
  (Rendering|SetVisibility (Variables|Default|GetJoyce_Mint) Selected false)
  (CallFunction|UdateCharacterData))

(event Custom|Selected%20Mint
  (params (Selected :type Boolean))
  (Variables|Default|SetSelected%20Skin 2)
  (Rendering|SetVisibility (Variables|Default|GetJoyce) Selected false)
  (Rendering|SetVisibility (Variables|Default|GetJoyce_Pink) Selected false)
  (Rendering|SetVisibility (Variables|Default|GetJoyce_Green) Selected false)
  (Rendering|SetVisibility (Variables|Default|GetJoyce_Mint) (not Selected) false)
  (CallFunction|UdateCharacterData))

(event EventBeginPlay
  (bind _returnvalue (UserInterface|CreateWidget "/Game/BluePrint/CharacterSelect/CharacterSelectionWidget.CharacterSelectionWidget_C" (Game|GetPlayerController 0)))
  (bind _output_get (Variables|Default|SetCharacterSelection%20widget _returnvalue))
  (Variables|/Game/BluePrint/CharacterSelect/CharacterSelectionWidget.CharacterSelectionWidget_C|SetCharacter%20selector _output_get self)
  (UserInterface|Viewport|AddtoViewport _output_get 0))

(event Collision|EventActorBeginOverlap
  (params (OtherActor :type Actor%20Object%20Reference)))

(event EventTick
  (params (DeltaSeconds :type Float%20%28single-precision%29)))

(fn ConstructionScript)