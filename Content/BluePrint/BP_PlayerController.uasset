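; Player controller for the KidKing game mode that requests the player's spawn and prints debug info.
; On BeginPlay, only a local controller fires a custom event, which casts the game mode to BP_KidKingGameMode and calls SpawnPlayer with itself.
; Tick runs through a one-second Delay to print the controlled pawn's display name roughly once per second.
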(event Custom|Custom%20Event
  (bind _asbp_kid_king_game_mode (Utilities|Casting|CastToBP_KidKingGameMode (Game|GetGameMode)))
  (Default|SpawnPlayer _asbp_kid_king_game_mode self))

(event EventBeginPlay
  (if (Pawn|IsLocalPlayerController)
    (CallFunction|CustomEvent)))

(event EventTick
  (params (DeltaSeconds :type Float%20%28single-precision%29))
  (Utilities|FlowControl|Delay 1.0)
  (Development|PrintString (Utilities|GetDisplayName (Pawn|GetControlledPawn))))

(fn ConstructionScript)