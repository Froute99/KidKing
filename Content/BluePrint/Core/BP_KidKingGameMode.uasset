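; KidKing game mode that tracks connected players, handles respawning and scores team area capture.
; Login, controller swap and logout events maintain the controller list, with login also assigning each BP_TestController its index.
; SpawnPlayer replaces a controller's pawn with a BP_NiceCleanCharacter at a random PlayerStart; Occupation adds delta time to red or blue capture points unless both teams are present.
; Widget creation and skin-based spawning remain as unconnected nodes.
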(event EventPostLogin
  (params (NewPlayer :type Player%20Controller%20Object%20Reference))
  (bind _returnvalue (Utilities|Array|Add (Variables|Default|GetPCs) NewPlayer))
  (bind _asbp_test_controller (Utilities|Casting|CastToBP_TestController NewPlayer))
  (bind _output_get (Variables|/Game/BluePrint/Core/BP_TestController.BP_TestController_C|SetIndex _asbp_test_controller _returnvalue))
  (Development|PrintString (Utilities|String|Append "Hello, " "Player" (Utilities|String|ToString(Integer) _output_get))))

(event EventBeginPlay
  (CallFunction|GetAllPlayerStarts))

(event EventOnLogout
  (params (ExitingController :type Controller%20Object%20Reference))
  (bind _asplayer_controller (Utilities|Casting|CastToPlayerController ExitingController))
  (Utilities|Array|RemoveItem (Variables|Default|GetPCs) _asplayer_controller))

(event EventOnSwapPlayerControllers
  (params (OldPC :type Player%20Controller%20Object%20Reference) (NewPC :type Player%20Controller%20Object%20Reference))
  (Utilities|Array|Add (Variables|Default|GetPCs) NewPC))

(fn ConstructionScript)

(fn Occupation
  (params (Array :type Array%20of%20Main%20Character%20Object%20References))
  (bind _returnvalue (Utilities|Time|GetWorldDeltaSeconds))
  (for _array_element Array
    (if (== (Variables|/Script/KidKing.MainCharacter|GetTeamCode _array_element) 0)
      (Variables|Default|SetIsRedTeam true)
      (else
        (Variables|Default|SetIsBlueTeam true))))
  (if (not (and (Variables|Default|GetIsRedTeam) (Variables|Default|GetIsBlueTeam)))
    (if (Variables|Default|GetIsRedTeam)
      ;[1 1 1] if True, red team gains point
      (Variables|Default|SetRedTeamCapturePoint (+ (Variables|Default|GetRedTeamCapturePoint) _returnvalue))
      (else
        ;[1 1 1] if True, blue team gains point
        (Variables|Default|SetBlueTeamCapturePoint (+ (Variables|Default|GetBlueTeamCapturePoint) _returnvalue))))))

(fn SpawnPlayer
  (params (Controller :type Controller%20Object%20Reference))
  (bind _returnvalue (Pawn|GetControlledPawn Controller))
  (Utilities|IsValid _returnvalue
    (:Is%20Valid
      (Actor|DestroyActor _returnvalue))
    (:Is%20Not%20Valid
      _))
  (bind _returnvalue_2 (Game|SpawnActorfromClass "/Game/BluePrint/MainCharacter/BP_NiceCleanCharacter.BP_NiceCleanCharacter_C" (Spawn|FindRandomStartPosition) "AdjustIfPossibleButAlwaysSpawn" 0 0))
  (Pawn|Possess Controller _returnvalue_2))

(fn FindRandomStartPosition
  (bind _outactors (Actor|GetAllActorsOfClass "/Script/Engine.PlayerStart"))
  (return (Transformation|GetActorTransform (Utilities|Array|Get(acopy) _outactors (Math|Random|RandomIntegerinRange 0 (- (Utilities|Array|Length _outactors) 1))))))

(fn GetAllPlayerStarts
  (bind _outactors (Actor|GetAllActorsOfClass "/Script/Engine.PlayerStart"))
  (Variables|Default|SetPlayerStarts _outactors))