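; Test player controller that requests a character spawn from BP_KidKingGameMode when play begins.
; On BeginPlay, the local controller calls RPCSpawnPlayer, and the RPC_SpawnPlayer event casts the game mode and passes itself to a spawn function.
; A switch offers Joyce at Player1Start or Sara with an empty start name, but its selector is hard-coded, so only the Sara branch runs.
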(event Custom|RPC_SpawnPlayer
  ;[0 0 0 1 60] Spawn Player
  (switch int 1
    (:0
      (bind _asbp_kid_king_game_mode (Utilities|Casting|CastToBP_KidKingGameMode (Game|GetGameMode)))
      (Default|SpawnJoyce _asbp_kid_king_game_mode self "Player1Start")
      (Development|PrintString "Spawn01"))
    (:1
      (bind _asbp_kid_king_game_mode_2 (Utilities|Casting|CastToBP_KidKingGameMode (Game|GetGameMode)))
      (Default|SpawnSara _asbp_kid_king_game_mode_2 self)
      (Development|PrintString "Spawn02"))))

(event EventBeginPlay
  ;[0 0 0 1 60] Spawn Player
  (if (Pawn|IsLocalPlayerController)
    (CallFunction|RPCSpawnPlayer)))

(event EventTick
  (params (DeltaSeconds :type Float%20%28single-precision%29)))

(fn ConstructionScript)