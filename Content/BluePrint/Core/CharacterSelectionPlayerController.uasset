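; Player controller for character selection that hosts and joins LAN multiplayer sessions.
; HostSession creates a four-connection LAN session, then opens stage_01 as a listen server.
; JoinSession searches for a single LAN session and joins the first result, with no empty-result check.
; Outcomes are reported through debug prints, though a failed search also prints the success message.
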(event Custom|Host%20Session
  (|Session self 4 true
    (:OnSuccess
      (Game|OpenLevel(byName) "stage_01" false "?listen"))
    (:OnFailure
      (Development|PrintString "Creating Session Fail"))))

(event Custom|Join%20Session
  (bind _results (|FindSessions self 1 true)
    (:OnSuccess
      (Development|PrintString "Finding Session Success")
      (|JoinSession self (Utilities|Array|Get(acopy) _results)
        (:OnSuccess
          (Development|PrintString "Join Success"))
        (:OnFailure
          (Development|PrintString "Join Fail"))))
    (:OnFailure
      (Development|PrintString "Finding Session Success"))))

(event EventBeginPlay)

(event EventTick
  (params (DeltaSeconds :type Float%20%28single-precision%29)))

(fn ConstructionScript)