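; Game state Blueprint that keeps score counters for two teams and notifies the UI when either changes.
; AddTeam1Score and AddTeam2Score each increment their team's counter, then share a call to UpdateScores.
; UpdateScores finds every widget implementing BPI_Score and sends it UpdateScoreMessage with only Team1Score, even after Team 2 scores.
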(event Custom|AddTeam2Score
  (bind _result (Math|Integer|IncrementInt (Variables|Score|GetTeam2Score))
    (:%20%20
      (Variables|Score|SetTeam2Score _result)
      (CallFunction|UpdateScores))))

(event Custom|AddTeam1Score
  (bind _result (Math|Integer|IncrementInt (Variables|Score|GetTeam1Score))
    (:%20%20
      (Variables|Score|SetTeam1Score _result)
      (CallFunction|UpdateScores))))

(event Custom|Update%20Scores
  (bind _foundwidgets (Class|WidgetBlueprintLibrary|GetAllWidgetswithInterface "/Game/BluePrint/Functions/BPI_Score.BPI_Score_C" false))
  (for _array_element _foundwidgets
    (Class|BPIScore|UpdateScore(Message) _array_element (Variables|Score|GetTeam1Score))))

(event EventBeginPlay)

(event EventTick
  (params (DeltaSeconds :type Float%20%28single-precision%29)))

(fn ConstructionScript)