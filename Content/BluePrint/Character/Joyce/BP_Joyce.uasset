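; Joyce player character with sword combos, dodge, run, guard and Spiral and Slash skills, plus camera shakes, death and boss health widgets, and debug keys.
; Input applies GAS effects and activates abilities by tag, while events here play montages, drive velocity timelines and spawn skill actors.
; A looping timer line-traces between sword sockets, with a DoOnce gating the damage effect and Character.Damaged event until UpdateNotify resets combo and trace.
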(event Custom|RPC_AnyDamage
  ;[1 1 1] Damaged
  (if (> (Class|BaseCharacter|GetHealth) 0.0)
    (Animation|PlayAnimMontage "/Game/BluePrint/Character/Joyce/Animation/Montage/Joyce_Hit.Joyce_Hit" 1.0 "None")))

(event Custom|CamShake
  (bind _returnvalue (Pawn|GetController))
  (bind _asplayer_controller (Utilities|Casting|CastToPlayerController _returnvalue))
  ;[1 1 1] CamShake
  (if (<= (Math|Vector|VectorLength (Transformation|GetVelocity)) 0.0)
    (Game|Feedback|ClientStartCameraShake _asplayer_controller "/Game/BluePrint/CamShake/IdleCamShake_BP.IdleCamShake_BP_C" 1.0 "CameraLocal" "0, 0, 0")
    (elif (>= (Math|Vector|VectorLength (Transformation|GetVelocity)) 301.0)
      (Game|Feedback|ClientStartCameraShake _asplayer_controller "/Game/BluePrint/CamShake/RunCamShake_BP.RunCamShake_BP_C" 1.0 "CameraLocal" "0, 0, 0")
      (else
        (Game|Feedback|ClientStartCameraShake _asplayer_controller "/Game/BluePrint/CamShake/WalkCamShake_BP.WalkCamShake_BP_C" 1.0 "CameraLocal" "0, 0, 0")))))

(event Custom|Btn%20Attack
  (bind _mesh (Variables|Character|GetMesh))
  ;[1 1 1] Default Attack
  ;;[0 0 0] Combo
  (if (Variables|Default|GetIsBtnAttack)
    (Variables|Default|SetIsBtnAttack false)
    (switch int (Variables|Default|GetComboIndex)
      (:0
        (Variables|Default|SetComboIndex 1)
        (Variables|Default|SetComboMoveDistance 1.5e+02)
        (Animation|Montage|PlayMontage _mesh "/Game/BluePrint/Character/Joyce/Animation/Montage/Combo1.Combo1"
          (:then
            (Timeline|Timeline PlayFromStart
              (:Update
                (Variables|/Script/Engine.MovementComponent|SetVelocity (Variables|Character|GetCharacterMovement) (Math|Vector|MakeVector (.x (* (Transformation|GetActorForwardVector) (Variables|Default|GetComboMoveDistance))) (.y (* (Transformation|GetActorForwardVector) (Variables|Default|GetComboMoveDistance))) (.z (Variables|/Script/Engine.MovementComponent|GetVelocity (Variables|Character|GetCharacterMovement))))))))
          (:OnInterrupted
            (Utilities|FlowControl|RetriggerableDelay 0.8 :!label _label)
            (CallFunction|UpdateNotify))))
      (:1
        (Variables|Default|SetComboIndex 2)
        (Variables|Default|SetComboMoveDistance 1e+03)
        (Animation|Montage|PlayMontage _mesh "/Game/BluePrint/Character/Joyce/Animation/Montage/Combo2.Combo2"
          (:then
            (Timeline|Timeline PlayFromStart))
          (:OnInterrupted
            (goto _label))))
      (:2
        (Variables|Default|SetComboIndex 3)
        (Variables|Default|SetComboMoveDistance 0.0)
        (Animation|Montage|PlayMontage _mesh "/Game/BluePrint/Character/Joyce/Animation/Montage/Combo3.Combo3"
          (:then
            (Timeline|Timeline PlayFromStart))
          (:OnInterrupted
            (goto _label))))
      (:3
        (Variables|Default|SetComboIndex 0)
        (Variables|Default|SetComboMoveDistance 1e+03)
        (Animation|Montage|PlayMontage _mesh "/Game/BluePrint/Character/Joyce/Animation/Montage/Combo4.Combo4"
          (:then
            (Timeline|Timeline PlayFromStart))
          (:OnInterrupted
            (goto _label)))))))

(event Custom|UpdateNotify
  ;[1 1 1] Default Attack
  (CallFunction|StopTriggerSword)
  (Input|EnableInput 0)
  (CallFunction|ResetCombo))

(event Custom|RPC_DebugHit
  ;[1 1 1] Debug Key
  ;;[0 0 0] Debug Hit
  (GameplayEffects|ApplyGameplayEffectToSelf :self (Variables|Default|GetAbilitySystemComponent) :GameplayEffectClass "/Game/BluePrint/Character/Joyce/Ability/Effects/GE_DamageSample.GE_DamageSample_C")
  (Ability|SendGameplayEventtoActor self "(TagName=\"Character.Damaged\")" (Utilities|Struct|MakeGameplayEventData "(TagName=\"Character.Damaged\")" self)))

(event Custom|TriggerSword
  ;[1 1 1] Default Attack
  ;;[0 0 0] Trace On
  (bind _returnvalue (Utilities|Time|SetTimerbyEvent (delegate Custom|SwordLineTrace) 0.01 true))
  (Variables|Default|SetTriggerSwordEvent _returnvalue))

(event Custom|SwordLineTrace
  (bind _staticmesh (Variables|Default|GetStaticMesh))
  ;[1 1 1] Default Attack
  (bind _outhit (Collision|LineTraceByChannel (Transformation|GetSocketLocation _staticmesh "BottomSocket") (Transformation|GetSocketLocation _staticmesh "TopSocket") "TraceTypeQuery3" false 0 "ForDuration"))
  (Utilities|IsValid (Ability|GetAbilitySystemComponent (.HitActor (Collision|BreakHitResult _outhit)))
    (:Is%20Valid
      (Utilities|FlowControl|DoOnce false
        (:Completed
          (GameplayEffects|ApplyGameplayEffectToTarget :self (Ability|GetAbilitySystemComponent (.HitActor (Collision|BreakHitResult _outhit))) :GameplayEffectClass "/Game/BluePrint/Character/Joyce/Ability/Effects/GE_DamageSample.GE_DamageSample_C" :Target (Ability|GetAbilitySystemComponent (.HitActor (Collision|BreakHitResult _outhit))))
          (Ability|SendGameplayEventtoActor (.HitActor (Collision|BreakHitResult _outhit)) "(TagName=\"Character.Damaged\")" (Utilities|Struct|MakeGameplayEventData "(TagName=\"\")" self (.HitActor (Collision|BreakHitResult _outhit)) 0 0 "()" "(GameplayTags=)" "(GameplayTags=)" 0.0 (Ability|TargetData|AbilityTargetDatafromActor (.HitActor (Collision|BreakHitResult _outhit))))))))))

(event Custom|StopTriggerSword
  ;[1 1 1] Default Attack
  ;;[0 0 0] Trace Off
  (Utilities|Time|ClearandInvalidateTimerbyHandle (Variables|Default|GetTriggerSwordEvent))
  (Utilities|FlowControl|DoOnce false) ; enters at Reset
)

(event Custom|Combo%20Attack
  (bind _mesh (Variables|Character|GetMesh))
  ;[1 1 1] Default Attack
  ;;[0 0 0] Combo
  (if (Variables|Default|GetIsAttackingCombo)
    (Variables|Default|SetIsBtnAttack true)
    (else
      (Variables|Default|SetIsAttackingCombo true)
      (switch int (Variables|Default|GetComboIndex)
        (:0
          (Variables|Default|SetComboIndex 1)
          (Variables|Default|SetComboMoveDistance 1.5e+02)
          (Animation|Montage|PlayMontage _mesh "/Game/BluePrint/Character/Joyce/Animation/Montage/Combo1.Combo1"
            (:then
              (Timeline|Timeline PlayFromStart
                (:Update
                  (Variables|/Script/Engine.MovementComponent|SetVelocity (Variables|Character|GetCharacterMovement) (Math|Vector|MakeVector (.x (* (Transformation|GetActorForwardVector) (Variables|Default|GetComboMoveDistance))) (.y (* (Transformation|GetActorForwardVector) (Variables|Default|GetComboMoveDistance))) (.z (Variables|/Script/Engine.MovementComponent|GetVelocity (Variables|Character|GetCharacterMovement))))))))
            (:OnInterrupted
              (Utilities|FlowControl|RetriggerableDelay 0.8 :!label _label)
              (CallFunction|UpdateNotify))))
        (:1
          (Variables|Default|SetComboIndex 2)
          (Variables|Default|SetComboMoveDistance 1e+03)
          (Animation|Montage|PlayMontage _mesh "/Game/BluePrint/Character/Joyce/Animation/Montage/Combo2.Combo2"
            (:then
              (Timeline|Timeline PlayFromStart))
            (:OnInterrupted
              (goto _label))))
        (:2
          (Variables|Default|SetComboIndex 3)
          (Variables|Default|SetComboMoveDistance 0.0)
          (Animation|Montage|PlayMontage _mesh "/Game/BluePrint/Character/Joyce/Animation/Montage/Combo3.Combo3"
            (:then
              (Timeline|Timeline PlayFromStart))
            (:OnInterrupted
              (goto _label))))
        (:3
          (Variables|Default|SetComboIndex 0)
          (Variables|Default|SetComboMoveDistance 1e+03)
          (Animation|Montage|PlayMontage _mesh "/Game/BluePrint/Character/Joyce/Animation/Montage/Combo4.Combo4"
            (:then
              (Timeline|Timeline PlayFromStart))
            (:OnInterrupted
              (goto _label))))))))

(event Custom|SlashSkill
  ;[1 1 1] Debug Key
  ;;[0 0 0] SlashSkill
  (Animation|Montage|PlayMontage (Variables|Character|GetMesh) "/Game/BluePrint/Character/Joyce/Animation/Montage/JoyceSlashSkill.JoyceSlashSkill"
    (:then
      (Input|DisableInput 0)
      (Utilities|FlowControl|Delay 2.0)
      (bind _returnvalue (Game|SpawnActorfromClass "/Game/BluePrint/Character/Joyce/Ability/BP_SlashSkill.BP_SlashSkill_C" (Math|Transform|MakeTransform (+ (Transformation|GetActorLocation) (* (Transformation|GetActorForwardVector) 2.5e+02)) "0, 0, 0" "1.000000,1.000000,1.000000") "AlwaysSpawn" self 0))
      (Input|EnableInput 0)
      (Utilities|FlowControl|Delay 2.0)
      (Actor|DestroyActor _returnvalue))))

(event Custom|Spiral
  (bind _returnvalue (Transformation|GetActorLocation))
  (bind _returnvalue_2 (Transformation|GetActorForwardVector))
  (bind _spiraldistance (Variables|Default|GetSpiralDistance))
  (bind _returnvalue_3 (* _returnvalue_2 _spiraldistance))
  ;[1 1 1] Debug Key
  ;;[0 0 0] Spiral
  (Animation|Montage|PlayMontage (Variables|Character|GetMesh) "/Game/BluePrint/Character/Joyce/Animation/Montage/JoyceSpiralSkill.JoyceSpiralSkill"
    (:then
      (Utilities|FlowControl|Delay 0.3)
      (bind _returnvalue_4 (Game|SpawnActorfromClass "/Game/BluePrint/Character/Joyce/Ability/BP_Thrust.BP_Thrust_C" (Math|Transform|MakeTransform (Math|Vector|MakeVector (.x _returnvalue) (.y _returnvalue) (.z _returnvalue)) (Transformation|GetActorRotation)) "Undefined" self 0))
      (Input|DisableInput 0)
      (Timeline|Timeline_0 PlayFromStart
        (:Update
          (Variables|/Script/Engine.MovementComponent|SetVelocity (Variables|Character|GetCharacterMovement) (Math|Vector|MakeVector (.x _returnvalue_3) (.y _returnvalue_3) (.z (Variables|/Script/Engine.MovementComponent|GetVelocity (Variables|Character|GetCharacterMovement)))))
          (Utilities|FlowControl|Delay 1.0)
          (Actor|DestroyActor _returnvalue_4)
          (Input|EnableInput 0))))))

(event Custom|ResetCombo
  ;[1 1 1] Default Attack
  ;;[0 0 0] Combo
  (Variables|Default|SetIsAttackingCombo false)
  (Variables|Default|SetIsBtnAttack false)
  (Variables|Default|SetComboIndex 0))

(event Input|EnhancedActionEvents|EnhancedInputActionIA_DebugAttack
  (params (ActionValue :type Boolean) (ElapsedSeconds :type Float%20%28double-precision%29) (TriggeredSeconds :type Float%20%28double-precision%29) (InputAction :type Input%20Action%20Object%20Reference :default "/Game/Input/Action/IA_DebugAttack.IA_DebugAttack"))
  ;[1 1 1] Default Attack
  ;;[0 0 0] Attack Key Bind
  (:Triggered
    (if (AI|Components|NavMovement|IsMovingonGround (Variables|Character|GetCharacterMovement))
      (Abilities|TryActivateAbilitiesbyTag (Variables|Default|GetAbilitySystemComponent) (Variables|GameplayTag|GetAttackTagContainer) true)
      (CallFunction|TriggerSword))))

(event Input|EnhancedActionEvents|EnhancedInputActionIA_Dodge
  (params (ActionValue :type Boolean) (ElapsedSeconds :type Float%20%28double-precision%29) (TriggeredSeconds :type Float%20%28double-precision%29) (InputAction :type Input%20Action%20Object%20Reference :default "/Game/Input/Action/IA_Dodge.IA_Dodge"))
  (bind _returnvalue (Transformation|GetActorForwardVector))
  (bind _movedistance (Variables|Default|GetMoveDistance))
  (bind _returnvalue_2 (* _returnvalue _movedistance))
  ;[1 1 1] Dodge
  (:Triggered
    (GameplayEffects|ApplyGameplayEffectToSelf :self (Variables|Default|GetAbilitySystemComponent) :GameplayEffectClass "/Game/BluePrint/Character/Joyce/Ability/Effects/GE_Dodge.GE_Dodge_C")
    (if (AI|Components|NavMovement|IsMovingonGround (Variables|Character|GetCharacterMovement))
      (Abilities|TryActivateAbilitiesbyTag (Variables|Default|GetAbilitySystemComponent) (Variables|GameplayTag|GetDodgeTagContainer) true)
      ;;[1 1 1] Don't Used
      (Timeline|Movement PlayFromStart
        (:Update
          (Variables|/Script/Engine.MovementComponent|SetVelocity (Variables|Character|GetCharacterMovement) (Math|Vector|MakeVector (.x _returnvalue_2) (.y _returnvalue_2) (.z (Variables|/Script/Engine.MovementComponent|GetVelocity (Variables|Character|GetCharacterMovement))))))))))

(event Input|EnhancedActionEvents|EnhancedInputActionIA_Run
  (params (ActionValue :type Boolean) (ElapsedSeconds :type Float%20%28double-precision%29) (TriggeredSeconds :type Float%20%28double-precision%29) (InputAction :type Input%20Action%20Object%20Reference :default "/Game/Input/Action/IA_Run.IA_Run"))
  ;[1 1 1] Debug Key
  (:Triggered
    (GameplayEffects|ApplyGameplayEffectToSelf :self (Variables|Default|GetAbilitySystemComponent) :GameplayEffectClass "/Game/BluePrint/Character/Joyce/Ability/Effects/GE_Run.GE_Run_C")
    (Abilities|TryActivateAbilitiesbyTag (Variables|Default|GetAbilitySystemComponent) (Variables|GameplayTag|GetRunTagContainer) true))
  (:Completed
    (Development|PrintString "Completed")
    (GameplayEffects|ApplyGameplayEffectToSelf :self (Variables|Default|GetAbilitySystemComponent) :GameplayEffectClass "/Game/BluePrint/Character/Joyce/Ability/Effects/GE_Walk.GE_Walk_C")
    (bind _returnvalue (Abilities|TryActivateAbilitiesbyTag (Variables|Default|GetAbilitySystemComponent) (Variables|GameplayTag|GetWalkTagContainer) true))
    (Development|PrintString (Utilities|String|ToString(Boolean) _returnvalue))))

(event EventBeginPlay
  ;[1 1 1] Init
  (bind _returnvalue (UserInterface|CreateWidget "/Game/BluePrint/UI/BP_WDG_BossHealthBar.BP_WDG_BossHealthBar_C"))
  (UserInterface|Viewport|AddtoViewport _returnvalue 0)
  (CallFunction|UpdateNotify))

(event EventOnDyingBP
  ;[1 1 1] Die
  (bind _returnvalue (UserInterface|CreateWidget "/Game/BluePrint/UI/BP_WDG_Death.BP_WDG_Death_C" (.AsPlayer%20Controller (Utilities|Casting|CastToPlayerController (Pawn|GetController)))))
  (UserInterface|Viewport|AddtoViewport _returnvalue 0))

(event EventTick
  (params (DeltaSeconds :type Float%20%28single-precision%29))
  ;[1 1 1] Tick
  (Utilities|FlowControl|Sequence
    (:then_0
      (CallFunction|CamShake)
      (Ability|Async|WaitGameplayEventToActor 0 "(TagName=\"Character.Damaged\")" true
        (:EventReceived
          (CallFunction|RPCAnyDamage))))))

(event Input|KeyboardEvents|DebugKeyF
  (params (Key :type Key%20Structure :default "None") (ActionValue :type Input%20Action%20Value%20Structure))
  ;[1 1 1] Debug Key
  ;;[0 0 0] SlashSkill
  (:Pressed
    (if (AI|Components|NavMovement|IsMovingonGround (Variables|Character|GetCharacterMovement))
      (Abilities|TryActivateAbilitiesbyTag (Variables|Default|GetAbilitySystemComponent) (Variables|GameplayTag|GetSlashTagContainer) true))))

(event Input|KeyboardEvents|DebugKeyG
  (params (Key :type Key%20Structure :default "None") (ActionValue :type Input%20Action%20Value%20Structure))
  ;[1 1 1] Debug Key
  ;;[0 0 0] Spiral
  (:Pressed
    (if (AI|Components|NavMovement|IsMovingonGround (Variables|Character|GetCharacterMovement))
      (Abilities|TryActivateAbilitiesbyTag (Variables|Default|GetAbilitySystemComponent) (Variables|GameplayTag|GetSpiralTagContainer) true))))

(event Input|KeyboardEvents|Subtract
  (params (Key :type Key%20Structure :default "None"))
  ;[1 1 1] Debug Key
  ;;[0 0 0] Debug Hit
  (:Pressed
    (CallFunction|RPCDebugHit)))

(event Input|MouseEvents|RightMouseButton
  (params (Key :type Key%20Structure :default "None"))
  (bind _charactermovement (Variables|Character|GetCharacterMovement))
  ;[1 1 1] Guard
  (:Pressed
    (if (not (or (AI|Components|NavMovement|IsFalling _charactermovement) (== (Variables|/Script/Engine.CharacterMovementComponent|GetMaxWalkSpeed _charactermovement) 9e+02)))
      (Variables|Default|SetIsBlocking true)
      (Variables|/Script/Engine.CharacterMovementComponent|SetMaxWalkSpeed (Variables|Character|GetCharacterMovement) 3e+02)
      (GameplayEffects|ApplyGameplayEffectToSelf :self (Variables|Default|GetAbilitySystemComponent) :GameplayEffectClass "/Game/BluePrint/Character/Joyce/Ability/Effects/GE_Guard.GE_Guard_C")
      (Development|SetHiddeninGame (Variables|Default|GetGuard) false false)))
  (:Released
    (Variables|Default|SetIsBlocking false)
    (Variables|/Script/Engine.CharacterMovementComponent|SetMaxWalkSpeed (Variables|Character|GetCharacterMovement) 6e+02)
    (GameplayEffects|RemoveActiveEffectswithTags (Variables|Default|GetAbilitySystemComponent) "(GameplayTags=((TagName=\"Ability.Guard\")))")
    (GameplayEffects|ApplyGameplayEffectToSelf :self (Variables|Default|GetAbilitySystemComponent) :GameplayEffectClass "/Game/BluePrint/Character/Joyce/Ability/Effects/GE_NoneGuard.GE_NoneGuard_C")))

(event Input|KeyboardEvents|Add
  (params (Key :type Key%20Structure :default "None"))
  ;[1 1 1] Debug Key
  ;;[0 0 0] Recover Health
)

(event Input|KeyboardEvents|Multiply
  (params (Key :type Key%20Structure :default "None"))
  ;[1 1 1] Debug Key
  ;;[0 0 0] Print Health & Stamina
  (:Pressed
    (Development|PrintString (Utilities|String|Append "Health: " (Utilities|String|ToString(Float) (Class|BaseCharacter|GetHealth))))
    (Development|PrintString (Utilities|String|Append "Stamina: " (Utilities|String|ToString(Float) (Class|BaseCharacter|GetStamina))))))

(fn ConstructionScript)

(fn HitCamShake
  (Camera|PlayWorldCameraShake "/Game/BluePrint/CamShake/HitCamShake_BP.HitCamShake_BP_C" (Transformation|GetActorLocation) 0.0 1e+03))

(fn GetCooldownPercentbyTag
  (params (Tags :type Gameplay%20Tag%20Container%20Structure))
  (bind _returnvalue (GameplayEffects|GetActiveEffectswithAllTags (Variables|Default|GetAbilitySystemComponent) Tags))
  (if (Utilities|Array|IsNotEmpty _returnvalue)
    (for _array_element _returnvalue
      (bind _returnvalue_2 (Ability|GameplayEffect|GetActiveGameplayEffectRemainingDuration _array_element))
      (return (/ _returnvalue_2 5.0)))))