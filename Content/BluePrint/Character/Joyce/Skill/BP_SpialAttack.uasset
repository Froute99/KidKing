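; BP_SpialAttack is a spiral attack skill actor for the Joyce character that follows her as an overlap volume.
; On BeginPlay it caches the first BP_Joyce found in the level.
; Every Tick it copies that character's location and rotation without sweeping.
; Its Capsule begin-overlap event only prints a debug hit message, with no damage or target filtering.
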(event OnComponentBeginOverlap(Capsule)
  (params (OverlappedComponent :type Primitive%20Component%20Object%20Reference) (OtherActor :type Actor%20Object%20Reference) (OtherComp :type Primitive%20Component%20Object%20Reference) (OtherBodyIndex :type Integer) (bFromSweep :type Boolean) (SweepResult :type Hit%20Result%20Structure%20%28by%20ref%29))
  (Development|PrintString "SprialAttack_Hit"))

(event EventBeginPlay
  (bind _outactors (Actor|GetAllActorsOfClass "/Game/BluePrint/Character/Joyce/BP_Joyce.BP_Joyce_C"))
  (Variables|Default|SetCharacter_REF (Utilities|Array|Get(acopy) _outactors)))

(event Collision|EventActorBeginOverlap
  (params (OtherActor :type Actor%20Object%20Reference)))

(event EventTick
  (params (DeltaSeconds :type Float%20%28single-precision%29))
  (bind _character_ref (Variables|Default|GetCharacter_REF))
  (bind _returnvalue (Transformation|GetActorLocation _character_ref))
  (Transformation|SetActorLocation (Math|Vector|MakeVector (.x _returnvalue) (.y _returnvalue) (.z _returnvalue)) false false)
  (Transformation|SetActorRotation (Transformation|GetActorRotation _character_ref)))

(fn ConstructionScript)