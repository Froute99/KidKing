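; BP_Thrust is a hitbox actor for Joyce's thrust ability that follows its owner's location and rotation every tick.
; Capsule overlaps with actors whose ability system component differs from the owner's print a debug hit message.
; They then call ApplyGameplayEffectToTarget on the owner's component with GE_DamageSample, though no target is wired.
; BeginPlay caches the first BP_Joyce found, but that reference is unused.
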(event OnComponentBeginOverlap(Capsule)
  (params (OverlappedComponent :type Primitive%20Component%20Object%20Reference) (OtherActor :type Actor%20Object%20Reference) (OtherComp :type Primitive%20Component%20Object%20Reference) (OtherBodyIndex :type Integer) (bFromSweep :type Boolean) (SweepResult :type Hit%20Result%20Structure%20%28by%20ref%29))
  (bind _returnvalue (Components|GetOwner))
  (bind _returnvalue_2 (Ability|GetAbilitySystemComponent _returnvalue))
  (if (!= _returnvalue_2 (Ability|GetAbilitySystemComponent OtherActor))
    (Development|PrintString "Thrust Hit")
    (GameplayEffects|ApplyGameplayEffectToTarget :self _returnvalue_2 :GameplayEffectClass "/Game/BluePrint/Character/Joyce/Ability/Effects/GE_DamageSample.GE_DamageSample_C")))

(event EventBeginPlay
  (bind _outactors (Actor|GetAllActorsOfClass "/Game/BluePrint/Character/Joyce/BP_Joyce.BP_Joyce_C"))
  (Variables|Default|SetCharacter_REF (Utilities|Array|Get(acopy) _outactors)))

(event Collision|EventActorBeginOverlap
  (params (OtherActor :type Actor%20Object%20Reference)))

(event EventTick
  (params (DeltaSeconds :type Float%20%28single-precision%29))
  (bind _returnvalue (Components|GetOwner))
  (bind _returnvalue_2 (Transformation|GetActorLocation _returnvalue))
  (Transformation|SetActorLocation (Math|Vector|MakeVector (.x _returnvalue_2) (.y _returnvalue_2) (.z _returnvalue_2)) false false)
  (Transformation|SetActorRotation (Transformation|GetActorRotation _returnvalue)))

(fn ConstructionScript)