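; BP_TestController is a test player controller that shows the main menu and handles player character spawning.
; BeginPlay creates the BP_WDG_MainMenu widget and adds it to the viewport.
; RPC_SpawnPlayer, if the controller is local, sets the game mode's HUD class, has BP_KidKingGameMode spawn the chosen character at Player1Start, then possesses it.
; Nothing in this graph triggers that event, as its only call here is disconnected.
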(event Custom|RPC_SpawnPlayer
  (params (Character%20Index :type Integer))
  ;[0 0 0] Spawn Player
  (if (Pawn|IsLocalPlayerController)
    (bind _asbp_kid_king_game_mode (Utilities|Casting|CastToBP_KidKingGameMode (Game|GetGameMode)))
    (Variables|/Script/Engine.GameModeBase|SetHUDClass _asbp_kid_king_game_mode "/Game/BluePrint/UI/BP_PlayerHUD.BP_PlayerHUD_C")
    (bind _returnvalue (Default|SpawnPlayer _asbp_kid_king_game_mode self "Player1Start" Character%20Index))
    (Pawn|Possess self _returnvalue)))

(event EventBeginPlay
  ;[0 0 0] Spawn Player
  (bind _returnvalue (UserInterface|CreateWidget "/Game/BluePrint/UI/BP_WDG_MainMenu.BP_WDG_MainMenu_C" self))
  (UserInterface|Viewport|AddtoViewport _returnvalue 0))

(fn ConstructionScript)