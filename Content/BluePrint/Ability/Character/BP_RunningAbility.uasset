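; BP_RunningAbility is a gameplay ability that makes a character run by raising its movement component's max walk speed.
; Activation is allowed only while the owner's ability system component has the Character.Run tag.
; On activation it commits and applies the faster speed, then sets a normal walk speed when the ability ends.
; Both speed changes print debug output, and the ability never ends itself.
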(event Custom|OnCommitAbility
  (bind _ascharacter_movement_component (Utilities|Casting|CastToCharacterMovementComponent (.MovementComponent (Utilities|Struct|BreakGameplayAbilityActorInfo (Ability|GetActorInfo))))
    (:then
      (bind _output_get (Variables|/Script/Engine.CharacterMovementComponent|SetMaxWalkSpeed _ascharacter_movement_component 1.2e+03))
      (Development|PrintString (Utilities|String|ToString(Float) _output_get)))
    (:CastFailed
      (Development|PrintString "Hello"))))

(event Ability|EventActivateAbility
  (Ability|CommitAbility)
  (CallFunction|OnCommitAbility))

(event Ability|EventOnEndAbility
  (params (bWasCancelled :type Boolean))
  (bind _ascharacter_movement_component (Utilities|Casting|CastToCharacterMovementComponent (.MovementComponent (Utilities|Struct|BreakGameplayAbilityActorInfo (Ability|GetActorInfo))))
    (:then
      (bind _output_get (Variables|/Script/Engine.CharacterMovementComponent|SetMaxWalkSpeed _ascharacter_movement_component 6e+02))
      (Development|PrintString (Utilities|String|ToString(Float) _output_get)))
    (:CastFailed
      (Development|PrintString "Hello"))))

(fn K2CanActivateAbility
  (params (ActorInfo :type Gameplay%20Ability%20Actor%20Info%20Structure) (Handle :type Gameplay%20Ability%20Spec%20Handle%20Structure))
  (return "" (GameplayTags|HasMatchingGameplayTag (.AbilitySystemComponent (Utilities|Struct|BreakGameplayAbilityActorInfo ActorInfo)) "(TagName=\"Character.Run\")")))