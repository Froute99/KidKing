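; Short-lived spike actor for the Golem ability that shoots up when spawned.
; BeginPlay quickly moves the capsule to a relative height of SpikeMaxHeight, destroys it after a pause, then destroys the actor shortly after.
; Overlapping BP_NiceCleanCharacter only prints a debug string, with no damage applied here; the stored InitialLocation is not read in this graph.
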(event EventBeginPlay
  (bind _capsule (Variables|Default|GetCapsule))
  (Variables|Default|SetInitialLocation (Transformation|GetActorLocation))
  (Components|MoveComponentTo _capsule (Math|Vector|MakeVectorNetQuantize 0.0 0.0 (Variables|Default|GetSpikeMaxHeight)) "0, 0, 0" false false 0.1 false)
  (Utilities|FlowControl|Delay 1.0)
  (Components|DestroyComponent _capsule)
  (Utilities|FlowControl|Delay 0.6)
  (Actor|DestroyActor))

(event Collision|EventActorBeginOverlap
  (params (OtherActor :type Actor%20Object%20Reference))
  (if (.bSuccess (Utilities|Casting|CastToBP_NiceCleanCharacter OtherActor))
    (Development|PrintString "Hello")))

(fn ConstructionScript)