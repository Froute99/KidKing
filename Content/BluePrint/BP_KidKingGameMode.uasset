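; King-of-the-hill style game mode that spawns the player's chosen character and scores team capture of a zone.
; BeginPlay reads the saved skin index from the game instance, spawns that character at a player start, and possesses it with player 0 after a short delay.
; Occupation checks occupants' team codes and adds frame time to red's points when only red is present, none when contested, and blue's otherwise, even with no occupants.
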(event EventBeginPlay
  (bind _skin_index (Class|InstanceInterface|LoadCharacterData(Message) (Game|GetGameInstance)))
  (bind _returnvalue (Game|SpawnActorfromClass (Utilities|Select :Index _skin_index :Option%200 "/Game/BluePrint/MainCharacter/Joyce/Joyce.Joyce_C" :Option%201 "/Game/BluePrint/MainCharacter/MyMainCharacter1.MyMainCharacter1_C" :Option%202 0) (Transformation|GetActorTransform (Class|GameModeBase|FindPlayerStart)) "Undefined" 0 0))
  (Utilities|FlowControl|Delay 0.2)
  (bind _as캐릭터 (Utilities|Casting|CastToCharacter _returnvalue))
  (Pawn|Possess (Game|GetPlayerController 0) _as캐릭터))

(event EventTick
  (params (DeltaSeconds :type Float%20%28single-precision%29)))

(fn ConstructionScript)

(fn Occupation
  (params (Array :type Array%20of%20My%20Main%20Character%201%20Object%20References))
  (bind _returnvalue (Utilities|Time|GetWorldDeltaSeconds))
  (for _array_element Array
    (if (== (Variables|/Game/BluePrint/MainCharacter/MyMainCharacter1.MyMainCharacter1_C|GetTeamCode _array_element) 0)
      (Variables|Default|SetIsRedTeam true)
      (else
        (Variables|Default|SetIsBlueTeam true))))
  (if (not (and (Variables|Default|GetIsRedTeam) (Variables|Default|GetIsBlueTeam)))
    (if (Variables|Default|GetIsRedTeam)
      ;[1 1 1] if True, red team gains point
      (Variables|Default|SetRedTeamCapturePoint (+ (Variables|Default|GetRedTeamCapturePoint) _returnvalue))
      (else
        ;[1 1 1] if True, blue team gains point
        (Variables|Default|SetBlueTeamCapturePoint (+ (Variables|Default|GetBlueTeamCapturePoint) _returnvalue))))))