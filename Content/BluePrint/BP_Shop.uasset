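; BP_Shop is a shop area actor that shows and hides a shop widget.
; Its Box overlap sets InShopArea when a Joyce-class actor enters.
; OpenShop lazily creates and caches Widget_Shop, then toggles it in the viewport without checking InShopArea.
; Any end overlap closes an open widget, and only in that case does a departing Joyce clear InShopArea.
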(event OnComponentBeginOverlap(Box)
  (params (OverlappedComponent :type Primitive%20Component%20Object%20Reference) (OtherActor :type Actor%20Object%20Reference) (OtherComp :type Primitive%20Component%20Object%20Reference) (OtherBodyIndex :type Integer) (bFromSweep :type Boolean) (SweepResult :type Hit%20Result%20Structure%20%28by%20ref%29))
  (if (Utilities|ClassIsChildOf (Utilities|GetClass OtherActor) "/Game/BluePrint/MainCharacter/Joyce/Joyce.Joyce_C")
    (Variables|Default|SetInShopArea true)))

(event OnComponentEndOverlap(Box)
  (params (OverlappedComponent :type Primitive%20Component%20Object%20Reference) (OtherActor :type Actor%20Object%20Reference) (OtherComp :type Primitive%20Component%20Object%20Reference) (OtherBodyIndex :type Integer))
  (bind _wdg_shop (Variables|Default|GetWDG_Shop))
  (Utilities|IsValid _wdg_shop
    (:Is%20Valid
      (if (UserInterface|Viewport|IsinViewport _wdg_shop)
        (Widget|RemovefromParent _wdg_shop)
        (if (Utilities|ClassIsChildOf (Utilities|GetClass OtherActor) "/Game/BluePrint/MainCharacter/Joyce/Joyce.Joyce_C")
          (Variables|Default|SetInShopArea false))))))

(event Custom|OpenShop
  (Utilities|IsValid (Variables|Default|GetWDG_Shop)
    (:Is%20Valid
      _)
    (:Is%20Not%20Valid
      (bind _returnvalue (UserInterface|CreateWidget "/Game/BluePrint/Widget_Shop.Widget_Shop_C"))
      (bind _output_get (Variables|Default|SetWDG_Shop _returnvalue))))
  (if (UserInterface|Viewport|IsinViewport _output_get)
    (Widget|RemovefromParent _output_get)
    (else
      (UserInterface|Viewport|AddtoViewport _output_get 0))))

(event EventBeginPlay)

(event Collision|EventActorBeginOverlap
  (params (OtherActor :type Actor%20Object%20Reference)))

(event EventTick
  (params (DeltaSeconds :type Float%20%28single-precision%29)))

(fn ConstructionScript)