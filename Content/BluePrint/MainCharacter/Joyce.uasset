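; Joyce is the player character, played with Joy-Con buttons and motion, plus keyboard and mouse bindings.
; Tick drives speed-based camera shake, accelerometer-swing attacks with rumble, and a Delay-gated stage countdown ending in next-stage or winner UI.
; Input handles stamina-based running, guarding, timeline-driven rolls, shop opening and a purchasable swing-triggered projectile skill.
; Death and respawn events toggle the death UI and input, alongside debug keys for HP, gold and items.
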(event Custom|IncreaseStamina
  ;[1 1 1] Run and Stamina
  (if (Variables|Default|GetCanIncreaseStamina)
    (Variables|Default|SetStamina (+ (Variables|Default|GetStamina) 2.0))
    (if (>= (Variables|Default|GetStamina) 1e+02)
      (Variables|Default|SetCanIncreaseStamina false)
      (else
        (Variables|Default|SetCanIncreaseStamina true)))))

(event Custom|Use%20Stamina
  ;[1 1 1] Run and Stamina
  (Variables|Default|SetStamina (- (Variables|Default|GetStamina) 2.0))
  (if (<= (Variables|Default|GetStamina) 0.0)
    (Variables|Default|SetisRunning false)
    (Variables|/Script/Engine.CharacterMovementComponent|SetMaxWalkSpeed (Variables|Character|GetCharacterMovement) 3e+02)
    (else
      (Development|PrintString (Utilities|String|ToString(Float) (Variables|Default|GetStamina))))))

(event Custom|Travel
  (Development|ExecuteConsoleCommand (Utilities|String|MakeLiteralString "ServerTravel /Game/Map/stage_01") 0)
  (Development|PrintString "Travel"))

(event Custom|Camera%20shake
  (bind _returnvalue (Game|GetPlayerController 0))
  ;[1 1 1] Run and Stamina
  (if (<= (Math|Vector|VectorLength (Transformation|GetVelocity)) 0.0)
    (Game|Feedback|ClientStartCameraShake _returnvalue "/Game/BluePrint/CamShake/IdleCamShake_BP.IdleCamShake_BP_C" 1.0 "CameraLocal" "0, 0, 0")
    (elif (>= (Math|Vector|VectorLength (Transformation|GetVelocity)) 301.0)
      (Game|Feedback|ClientStartCameraShake _returnvalue "/Game/BluePrint/CamShake/RunCamShake_BP.RunCamShake_BP_C" 1.0 "CameraLocal" "0, 0, 0")
      (else
        (Game|Feedback|ClientStartCameraShake _returnvalue "/Game/BluePrint/CamShake/WalkCamShake_BP.WalkCamShake_BP_C" 1.0 "CameraLocal" "0, 0, 0")))))

(event Input|EnhancedActionEvents|EnhancedInputActionSkill_R
  (params (ActionValue :type Boolean) (ElapsedSeconds :type Float%20%28double-precision%29) (TriggeredSeconds :type Float%20%28double-precision%29) (InputAction :type Input%20Action%20Object%20Reference :default "/Game/Input/Action/Skill_R.Skill_R"))
  (bind _self self)
  ;[1 1 1] Remember this key will be changed in an action key mapping
  (:Triggered
    (if (Variables|Default|GetIsSkillPurchased)
      (if (< (.X (Class|KismetMathLibrary|BreakVector3f (.Accelerometer (Class|JoyConDriverFunctionLibrary|GetJoyConAccelerometer 1)))) -2.0)
        (Utilities|FlowControl|Delay 0.5)
        (bind _returnvalue (Game|SpawnActorfromClass "/Game/BluePrint/Ability/BP_FireballProjectile.BP_FireballProjectile_C" (Transformation|GetActorTransform _self) "Undefined" 0 _self))
        (Niagara|SetNiagaraVariable(Vector3) (Variables|/Game/BluePrint/Ability/BP_FireballProjectile.BP_FireballProjectile_C|GetNiagara _returnvalue) "SlashVector" (Math|Vector|RotateVectorAroundAxis (Transformation|GetActorForwardVector) -9e+01 "0.000000,0.000000,1.000000"))
        (Niagara|SetNiagaraVariable(Vector3) (Variables|/Game/BluePrint/Ability/BP_FireballProjectile.BP_FireballProjectile_C|GetNiagara _returnvalue) "Velocity" (* (Transformation|GetActorForwardVector) 8e+02))))))

(event EventOnRespawn
  ;[1 1 1] Respawn
  (Widget|RemovefromParent (Variables|Default|GetDie_UI))
  (Input|EnableInput (Game|GetPlayerController 0)))

(event Collision|EventActorBeginOverlap
  (params (OtherActor :type Actor%20Object%20Reference)))

(event EventTick
  (params (DeltaSeconds :type Float%20%28single-precision%29))
  (bind _returnvalue (Game|GetPlayerController 0))
  (bind _returnvalue_2 (Game|GetPlayerController 0))
  ;[1 1 1] Accelerometer Attack
  (CallFunction|CameraShake)
  (if (and (< (.X (Class|KismetMathLibrary|BreakVector3f (.Accelerometer (Class|JoyConDriverFunctionLibrary|GetJoyConAccelerometer 1)))) -1.0) (not (Variables|Default|GetIsAttacking)))
    (Variables|Default|SetAcell true)
    (Variables|Default|SetIsAttacking true)
    (if true
      (Animation|PlayAnimMontage "/Game/BluePrint/MainCharacter/Montage/JoyceAttack.JoyceAttack" 1.0 "")
      (bind _outactors (Actor|GetAllActorsOfClass "/Game/BluePrint/MainCharacter/Weapon_BP.Weapon_BP_C"))
      (bind _output_get (Variables|Default|SetWeapon (Utilities|Array|Get(acopy) _outactors)))
      (if (Variables|/Game/BluePrint/MainCharacter/Weapon_BP.Weapon_BP_C|Getactivated _output_get)
        (Class|JoyConDriverFunctionLibrary|SetJoyConRumble 1 1.6e+02 3.2e+02 0.6 50)
        ;[1 1 1] Timer
        (Utilities|FlowControl|Delay 1.0 :!label _label)
        (if (== (Variables|Default|GetSeconds) 0)
          (if (== (Variables|Default|GetMinute) 0)
            ;[1 1 1] Switch Timeup UI
            (bind _returnvalue_3 (Game|GetCurrentLevelName true))
            (if (Utilities|Enum|Equal(Enum) (Utilities|Text|ToText(String) _returnvalue_3) (Utilities|Text|ToText(String) (Variables|Default|GetStage_01)))
              (Variables|/Script/Engine.PlayerController|SetbShowMouseCursor _returnvalue_2 true)
              (Input|SetInputModeUIOnly _returnvalue_2 0 "DoNotLock" false)
              (bind _returnvalue_4 (UserInterface|CreateWidget "/Game/BluePrint/UI/NextStage.NextStage_C"))
              (bind _output_get_2 (Variables|Default|SetNextStage_UI _returnvalue_4))
              (UserInterface|Viewport|AddtoViewport _output_get_2 0)
              (else
                (Variables|/Script/Engine.PlayerController|SetbShowMouseCursor _returnvalue true)
                (Input|SetInputModeUIOnly _returnvalue 0 "DoNotLock" false)
                (bind _returnvalue_5 (UserInterface|CreateWidget "/Game/BluePrint/UI/FinalStageWinner.FinalStageWinner_C"))
                (bind _output_get_3 (Variables|Default|SetFinalStage_UI _returnvalue_5))
                (UserInterface|Viewport|AddtoViewport _output_get_3 0)))
            (else
              (Variables|Default|SetSeconds 59)
              (Variables|Default|SetMinute (- (Variables|Default|GetMinute) 1))))
          (else
            (Variables|Default|SetSeconds (- (Variables|Default|GetSeconds) 1))))))
    (else
      (Variables|Default|SetAcell false)
      (Variables|Default|SetIsAttacking false)
      (goto _label))))

(event EventOnCharacterDie
  ;[1 1 1] Respawn
  (bind _returnvalue (UserInterface|CreateWidget "/Game/BluePrint/UI/DieUI_BP.DieUI_BP_C"))
  (bind _output_get (Variables|Default|SetDie_UI _returnvalue))
  (UserInterface|Viewport|AddtoViewport _output_get 0)
  (Input|DisableInput (Game|GetPlayerController 0))
  (Widget|SetKeyboardFocus (Variables|Default|GetDie_UI)))

(event EventBeginPlay
  ;[1 1 1] MiniMap
  (bind _as플레이어_컨트롤러 (Utilities|Casting|CastToPlayerController (Pawn|GetController)))
  (Utilities|IsValid (PlayerController|LocalPlayerSubsystems|GetEnhancedInputLocalPlayerSubsystem _as플레이어_컨트롤러)
    (:Is%20Valid
      (Input|AddMappingContext (PlayerController|LocalPlayerSubsystems|GetEnhancedInputLocalPlayerSubsystem _as플레이어_컨트롤러) "/Game/Input/NewInputMappingContext.NewInputMappingContext" 0 "(bIgnoreAllPressedKeysUntilRelease=True,bForceImmediately=False)")
      ;[1 1 1] Shop Setter
      (bind _outactors (Actor|GetAllActorsOfClass "/Game/BluePrint/BP_Shop.BP_Shop_C"))
      (Variables|Default|SetShop (Utilities|Array|Get(acopy) _outactors)))))

(event Input|KeyboardEvents|DebugKeySubtract
  (params (Key :type Key%20Structure :default "None") (ActionValue :type Input%20Action%20Value%20Structure))
  ;[1 1 1] Debug
)

(event Input|KeyboardEvents|DebugKeyJoyConB
  (params (Key :type Key%20Structure :default "None") (ActionValue :type Input%20Action%20Value%20Structure))
  ;[1 1 1] Run and Stamina
  (:Released
    (if (not (Variables|Default|GetIsBlocking))
      (Variables|Default|SetisRunning false)
      (Variables|Default|SetCanIncreaseStamina true)
      (Variables|/Script/Engine.CharacterMovementComponent|SetMaxWalkSpeed (Variables|Character|GetCharacterMovement) 3e+02 :!label _label)
      (Utilities|FlowControl|RetriggerableDelay 0.2)
      (CallFunction|IncreaseStamina)
      (if (Variables|Default|GetCanIncreaseStamina)
        (goto _label)))))

(event Input|KeyboardEvents|DebugKeyG
  (params (Key :type Key%20Structure :default "None") (ActionValue :type Input%20Action%20Value%20Structure))
  ;[1 1 1] Remember this key will be changed in an action key mapping
)

(event Input|KeyboardEvents|DebugKeyH
  (params (Key :type Key%20Structure :default "None") (ActionValue :type Input%20Action%20Value%20Structure))
  ;[1 1 1] Remember this key will be changed in an action key mapping
)

(event Input|KeyboardEvents|DebugKeyJ
  (params (Key :type Key%20Structure :default "None") (ActionValue :type Input%20Action%20Value%20Structure))
  ;[1 1 1] Debug
)

(event Input|KeyboardEvents|DebugKeyJoyConA
  (params (Key :type Key%20Structure :default "None") (ActionValue :type Input%20Action%20Value%20Structure))
  ;[1 1 1] Remember this key will be changed in an action key mapping
)

(event Input|KeyboardEvents|LeftShift
  (params (Key :type Key%20Structure :default "None"))
  ;[1 1 1] Run and Stamina
  (:Pressed
    (if (not (Variables|Default|GetIsBlocking))
      (Variables|Default|SetisRunning true)
      (Variables|Default|SetCanIncreaseStamina false)
      (Variables|/Script/Engine.CharacterMovementComponent|SetMaxWalkSpeed (Variables|Character|GetCharacterMovement) 6e+02 :!label _label)
      (Utilities|FlowControl|RetriggerableDelay 0.2)
      (CallFunction|UseStamina)
      (if (Variables|Default|GetisRunning)
        (goto _label))))
  (:Released
    (if (not (Variables|Default|GetIsBlocking))
      (Variables|Default|SetisRunning false)
      (Variables|Default|SetCanIncreaseStamina true)
      (Variables|/Script/Engine.CharacterMovementComponent|SetMaxWalkSpeed (Variables|Character|GetCharacterMovement) 3e+02 :!label _label_2)
      (Utilities|FlowControl|RetriggerableDelay 0.2)
      (CallFunction|IncreaseStamina)
      (if (Variables|Default|GetCanIncreaseStamina)
        (goto _label_2)))))

(event Input|MouseEvents|RightMouseButton
  (params (Key :type Key%20Structure :default "None"))
  ;[1 1 1] Guard
  (:Pressed
    (if (not (or (AI|Components|NavMovement|IsFalling (Variables|Character|GetCharacterMovement)) (== (Variables|Default|GetisRunning) true)))
      (Variables|Default|SetIsBlocking true)
      (Variables|/Script/Engine.CharacterMovementComponent|SetMaxWalkSpeed (Variables|Character|GetCharacterMovement) 1e+02)
      (Development|SetHiddeninGame (Variables|Default|GetGuard) false false)))
  (:Released
    (Variables|Default|SetIsBlocking false)
    (Variables|/Script/Engine.CharacterMovementComponent|SetMaxWalkSpeed (Variables|Character|GetCharacterMovement) 3e+02)
    (Development|SetHiddeninGame (Variables|Default|GetGuard) true false)))

(event Input|MouseEvents|MouseWheelDown
  (params (Key :type Key%20Structure :default "None"))
  (:Pressed
    (if (not (Variables|Default|GetISMovementRoll))
      (Variables|Default|SetISMovementRoll true)
      (Animation|Montage|PlayMontage (Variables|Character|GetMesh) "/Game/BluePrint/MainCharacter/Montage/Rolling.Rolling"
        (:then
          (bind _distancemultiplier (Timeline|Movement PlayFromStart)
            (:Update
              (Variables|/Script/Engine.MovementComponent|SetVelocity (Variables|Character|GetCharacterMovement) (Math|Vector|MakeVector (.x (* (Transformation|GetActorForwardVector) (* _distancemultiplier (Variables|Default|GetMoveDistance)))) (.y (* (Transformation|GetActorForwardVector) (* _distancemultiplier (Variables|Default|GetMoveDistance)))) (.z (Variables|/Script/Engine.MovementComponent|GetVelocity (Variables|Character|GetCharacterMovement))))))))
        (:OnCompleted
          (Variables|Default|SetISMovementRoll false))))))

(event Input|KeyboardEvents|JoyConL
  (params (Key :type Key%20Structure :default "None"))
  (:Pressed
    (if (not (Variables|Default|GetISMovementRoll))
      (Variables|Default|SetISMovementRoll true)
      (Animation|Montage|PlayMontage (Variables|Character|GetMesh) "/Game/BluePrint/MainCharacter/Montage/Rolling.Rolling"
        (:then
          (bind _distancemultiplier (Timeline|Movement PlayFromStart)
            (:Update
              (Variables|/Script/Engine.MovementComponent|SetVelocity (Variables|Character|GetCharacterMovement) (Math|Vector|MakeVector (.x (* (Transformation|GetActorForwardVector) (* _distancemultiplier (Variables|Default|GetMoveDistance)))) (.y (* (Transformation|GetActorForwardVector) (* _distancemultiplier (Variables|Default|GetMoveDistance)))) (.z (Variables|/Script/Engine.MovementComponent|GetVelocity (Variables|Character|GetCharacterMovement))))))))
        (:OnCompleted
          (Variables|Default|SetISMovementRoll false))))))

(event Input|KeyboardEvents|JoyConB
  (params (Key :type Key%20Structure :default "None"))
  (:Pressed
    ;[1 1 1] Run and Stamina
    (if (not (Variables|Default|GetIsBlocking))
      (Variables|Default|SetisRunning true)
      (Variables|Default|SetCanIncreaseStamina false)
      (Variables|/Script/Engine.CharacterMovementComponent|SetMaxWalkSpeed (Variables|Character|GetCharacterMovement) 6e+02 :!label _label)
      (Utilities|FlowControl|RetriggerableDelay 0.2)
      (CallFunction|UseStamina)
      (if (Variables|Default|GetisRunning)
        (goto _label))))
  (:Released
    (if (not (Variables|Default|GetIsBlocking))
      (Variables|Default|SetisRunning false)
      (Variables|Default|SetCanIncreaseStamina true)
      (Variables|/Script/Engine.CharacterMovementComponent|SetMaxWalkSpeed (Variables|Character|GetCharacterMovement) 3e+02 :!label _label_2)
      (Utilities|FlowControl|RetriggerableDelay 0.2)
      (CallFunction|IncreaseStamina)
      (if (Variables|Default|GetCanIncreaseStamina)
        (goto _label_2)))))

(event Input|KeyboardEvents|F
  (params (Key :type Key%20Structure :default "None"))
  (bind _self self)
  ;[1 1 1] Remember this key will be changed in an action key mapping
  (:Pressed
    (bind _returnvalue (Game|SpawnActorfromClass "/Game/BluePrint/Ability/BP_FireballProjectile.BP_FireballProjectile_C" (Transformation|GetActorTransform _self) "Undefined" 0 _self))
    (Niagara|SetNiagaraVariable(Vector3) (Variables|/Game/BluePrint/Ability/BP_FireballProjectile.BP_FireballProjectile_C|GetNiagara _returnvalue) "SlashVector" (Math|Vector|RotateVectorAroundAxis (Transformation|GetActorForwardVector) -9e+01 "0.000000,0.000000,1.000000"))
    (Niagara|SetNiagaraVariable(Vector3) (Variables|/Game/BluePrint/Ability/BP_FireballProjectile.BP_FireballProjectile_C|GetNiagara _returnvalue) "Velocity" (* (Transformation|GetActorForwardVector) 8e+02))))

(event Input|KeyboardEvents|JoyConZl
  (params (Key :type Key%20Structure :default "None"))
  ;[1 1 1] Guard
  (:Pressed
    (if (not (or (AI|Components|NavMovement|IsFalling (Variables|Character|GetCharacterMovement)) (== (Variables|Default|GetisRunning) true)))
      (Variables|Default|SetIsBlocking true)
      (Variables|/Script/Engine.CharacterMovementComponent|SetMaxWalkSpeed (Variables|Character|GetCharacterMovement) 1e+02)
      (Development|SetHiddeninGame (Variables|Default|GetGuard) false false)))
  (:Released
    (Variables|Default|SetIsBlocking false)
    (Variables|/Script/Engine.CharacterMovementComponent|SetMaxWalkSpeed (Variables|Character|GetCharacterMovement) 3e+02)
    (Development|SetHiddeninGame (Variables|Default|GetGuard) true false)))

(event Input|KeyboardEvents|JoyConA
  (params (Key :type Key%20Structure :default "None"))
  ;[1 1 1] Remember this key will be changed in an action key mapping
  (:Pressed
    (if (Variables|Default|GetCan%20Use%20Shop)
      (Input|SetInputModeUIOnly (Game|GetPlayerController 0) 0 "DoNotLock" false)
      (bind _foundwidgets (Widget|GetAllWidgetsOfClass "/Game/BluePrint/UI/BP_WDG_Shop.BP_WDG_Shop_C" true))
      (bind _output_get (Variables|Default|SetShop%20widget (Utilities|Array|Get(acopy) _foundwidgets)))
      (Widget|SetKeyboardFocus _output_get)
      (Default|OpenShop (Variables|Default|GetShop)))))

(event Input|KeyboardEvents|Subtract
  (params (Key :type Key%20Structure :default "None"))
  ;[1 1 1] Debug
  (:Pressed
    (Class|CharacterBase|DebugDecreaseHp)))

(event Input|KeyboardEvents|J
  (params (Key :type Key%20Structure :default "None"))
  ;[1 1 1] Debug
  (:Pressed
    (for _array_element (Variables|Default|GetItems)
      (Development|PrintString (Utilities|String|ToString(Name) (Variables|/Script/KidKing.ItemInterface|GetItemName _array_element))))))

(event Input|KeyboardEvents|G
  (params (Key :type Key%20Structure :default "None"))
  ;[1 1 1] Remember this key will be changed in an action key mapping
  (:Pressed
    (if (Variables|Default|GetCan%20Use%20Shop)
      (Input|SetInputModeUIOnly (Game|GetPlayerController 0) 0 "DoNotLock" false)
      (bind _foundwidgets (Widget|GetAllWidgetsOfClass "/Game/BluePrint/UI/BP_WDG_Shop.BP_WDG_Shop_C" true))
      (bind _output_get (Variables|Default|SetShop%20widget (Utilities|Array|Get(acopy) _foundwidgets)))
      (Widget|SetKeyboardFocus _output_get)
      (Default|OpenShop (Variables|Default|GetShop)))))

(event Input|KeyboardEvents|H
  (params (Key :type Key%20Structure :default "None"))
  ;[1 1 1] Remember this key will be changed in an action key mapping
  (:Pressed
    (Variables|Default|SetGold (+ (Variables|Default|GetGold) 1e+01))))

(fn ConstructionScript
  (Variables|Default|SetCan%20Use%20Shop true))

(fn CamShake
  (Camera|PlayWorldCameraShake "/Game/BluePrint/CamShake/HitCamShake_BP.HitCamShake_BP_C" (Transformation|GetActorLocation) 0.0 1e+03))