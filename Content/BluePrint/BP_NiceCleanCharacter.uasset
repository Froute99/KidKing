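; Player character Blueprint for melee combat, using GAS tag-activated abilities for dodge and attack, plus a right-mouse guard that changes walk speed.
; A looping timer line-traces between sword sockets, with a DoOnce gating the damage effect and Character.Damaged event sent to targets.
; Tick picks idle, walk or run camera shake by speed and registers a damage-event wait that triggers health update and hit montage.
; Debug keys self-damage or initialise the health widget.
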(event Custom|RPC_AnyDamage
  ;[1 1 1 1 60] Damaged
  (Class|NiceCleanCharacter|UpdateHealth 1e+01)
  (Animation|PlayAnimMontage "/Game/BluePrint/MainCharacter/Joyce/JoyceOrigin/Joyce_Hit.Joyce_Hit" 1.0 "None"))

(event Custom|CamShake
  (bind _returnvalue (Pawn|GetController))
  (bind _asplayer_controller (Utilities|Casting|CastToPlayerController _returnvalue))
  ;[1 1 1] CamShake
  (if (<= (Math|Vector|VectorLength (Transformation|GetVelocity)) 0.0)
    (Game|Feedback|ClientStartCameraShake _asplayer_controller "/Game/BluePrint/CamShake/IdleCamShake_BP.IdleCamShake_BP_C" 1.0 "CameraLocal" "0, 0, 0")
    (elif (>= (Math|Vector|VectorLength (Transformation|GetVelocity)) 301.0)
      (Game|Feedback|ClientStartCameraShake _asplayer_controller "/Game/BluePrint/CamShake/RunCamShake_BP.RunCamShake_BP_C" 1.0 "CameraLocal" "0, 0, 0")
      (else
        (Game|Feedback|ClientStartCameraShake _asplayer_controller "/Game/BluePrint/CamShake/WalkCamShake_BP.WalkCamShake_BP_C" 1.0 "CameraLocal" "0, 0, 0")))))

(event Custom|RPC_DebugHit
  ;[1 1 1 1 60] Debug Key
  (GameplayEffects|ApplyGameplayEffectToSelf :self (Variables|Default|GetAbilitySystemComponent) :GameplayEffectClass "/Game/BluePrint/Ability/BP_GAS_DamageEffect.BP_GAS_DamageEffect_C")
  (Ability|SendGameplayEventtoActor self "(TagName=\"Character.Damaged\")" (Utilities|Struct|MakeGameplayEventData "(TagName=\"Character.Damaged\")" self)))

(event Custom|TriggerSword
  ;[1 1 1 1 60] Default Attack
  ;;[0 0 0 1 36] Trace On
  (bind _returnvalue (Utilities|Time|SetTimerbyEvent (delegate Custom|SwordLineTrace) 0.01 true))
  (Variables|Default|SetTriggerSwordEvent _returnvalue))

(event Custom|SwordLineTrace
  (bind _sword (Variables|Default|GetSword))
  ;[1 1 1 1 60] Default Attack
  (bind _outhit (Collision|LineTraceByChannel (Transformation|GetSocketLocation _sword "Bottom") (Transformation|GetSocketLocation _sword "Top") "TraceTypeQuery3" false 0 "ForDuration"))
  (Utilities|IsValid (Ability|GetAbilitySystemComponent (.HitActor (Collision|BreakHitResult _outhit)))
    (:Is%20Valid
      (Utilities|FlowControl|DoOnce false
        (:Completed
          (GameplayEffects|ApplyGameplayEffectToTarget :self (Variables|Default|GetAbilitySystemComponent) :GameplayEffectClass "/Game/BluePrint/Ability/BP_GAS_DamageEffect.BP_GAS_DamageEffect_C" :Target (Ability|GetAbilitySystemComponent (.HitActor (Collision|BreakHitResult _outhit))))
          (Ability|SendGameplayEventtoActor (.HitActor (Collision|BreakHitResult _outhit)) "(TagName=\"Character.Damaged\")" (Utilities|Struct|MakeGameplayEventData "(TagName=\"\")" self (.HitActor (Collision|BreakHitResult _outhit)) 0 0 "()" "(GameplayTags=)" "(GameplayTags=)" 0.0 (Ability|TargetData|AbilityTargetDatafromActor (.HitActor (Collision|BreakHitResult _outhit))))))))))

(event Custom|StopTriggerSword
  ;[1 1 1 1 60] Default Attack
  ;;[0 0 0 1 36] Trace Off
  (Utilities|Time|ClearandInvalidateTimerbyHandle (Variables|Default|GetTriggerSwordEvent))
  (Utilities|FlowControl|DoOnce false) ; enters at Reset
)

(event Input|EnhancedActionEvents|EnhancedInputActionIA_DebugAttack
  (params (ActionValue :type Boolean) (ElapsedSeconds :type Float%20%28double-precision%29) (TriggeredSeconds :type Float%20%28double-precision%29) (InputAction :type Input%20Action%20Object%20Reference :default "/Game/Input/Action/IA_DebugAttack.IA_DebugAttack"))
  ;[1 1 1 1 60] Default Attack
  ;;[0 0 0 1 36] Attack Key Bind
  (:Triggered
    (if (AI|Components|NavMovement|IsMovingonGround (Variables|Character|GetCharacterMovement))
      (Abilities|TryActivateAbilitiesbyTag (Variables|Default|GetAbilitySystemComponent) (Variables|Default|GetAttackTagContainer) true))))

(event Input|EnhancedActionEvents|EnhancedInputActionIA_Dodge
  (params (ActionValue :type Boolean) (ElapsedSeconds :type Float%20%28double-precision%29) (TriggeredSeconds :type Float%20%28double-precision%29) (InputAction :type Input%20Action%20Object%20Reference :default "/Game/Input/Action/IA_Dodge.IA_Dodge"))
  (bind _returnvalue (Transformation|GetActorForwardVector))
  (bind _movedistance (Variables|Default|GetMoveDistance))
  (bind _returnvalue_2 (* _returnvalue _movedistance))
  ;[1 1 1] Dodge
  (:Triggered
    (if (AI|Components|NavMovement|IsMovingonGround (Variables|Character|GetCharacterMovement))
      (Abilities|TryActivateAbilitiesbyTag (Variables|Default|GetAbilitySystemComponent) (Variables|Default|GetDodgeTagContainer) true)
      (Timeline|Movement PlayFromStart
        (:Update
          (Variables|/Script/Engine.MovementComponent|SetVelocity (Variables|Character|GetCharacterMovement) (Math|Vector|MakeVector (.x _returnvalue_2) (.y _returnvalue_2) (.z (Variables|/Script/Engine.MovementComponent|GetVelocity (Variables|Character|GetCharacterMovement))))))))))

(event EventBeginPlay
  ;[1 1 1 1 60] Init
)

(event EventTick
  (params (DeltaSeconds :type Float%20%28single-precision%29))
  ;[1 1 1 1 60] Tick
  (CallFunction|CamShake)
  (Ability|Async|WaitGameplayEventToActor 0 "(TagName=\"Character.Damaged\")" true
    (:EventReceived
      (CallFunction|RPCAnyDamage))))

(event Input|KeyboardEvents|Subtract
  (params (Key :type Key%20Structure))
  ;[1 1 1 1 60] Debug Key
  (:Pressed
    (CallFunction|RPCDebugHit)))

(event Input|MouseEvents|RightMouseButton
  (params (Key :type Key%20Structure))
  (bind _charactermovement (Variables|Character|GetCharacterMovement))
  ;[1 1 1] Guard
  (:Pressed
    (if (not (or (AI|Components|NavMovement|IsFalling _charactermovement) (== (Variables|/Script/Engine.CharacterMovementComponent|GetMaxWalkSpeed _charactermovement) 9e+02)))
      (Variables|Default|SetIsBlocking true)
      (Variables|/Script/Engine.CharacterMovementComponent|SetMaxWalkSpeed (Variables|Character|GetCharacterMovement) 3e+02)
      (Development|SetHiddeninGame (Variables|Default|GetGuard) false false)))
  (:Released
    (Variables|Default|SetIsBlocking false)
    (Variables|/Script/Engine.CharacterMovementComponent|SetMaxWalkSpeed (Variables|Character|GetCharacterMovement) 6e+02)
    (Development|SetHiddeninGame (Variables|Default|GetGuard) true false)))

(event Input|KeyboardEvents|Add
  (params (Key :type Key%20Structure))
  ;[1 1 1 1 60] Debug Key
  (:Pressed
    (Class|NiceCleanCharacter|InitHealthWidget)))

(fn ConstructionScript)

(fn AttachHpSpWidget
  (params (Controller :type Controller%20Object%20Reference))
  (bind _returnvalue (UserInterface|CreateWidget "/Game/BluePrint/UI/BP_PlayerWidget.BP_PlayerWidget_C" (.AsBP%20Test%20Controller (Utilities|Casting|CastToBP_TestController Controller))))
  (bind _output_get (Variables|Default|SetPlayerWidget _returnvalue))
  (UserInterface|Viewport|AddtoPlayerScreen _output_get))